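; BP_SkillBallTray is a tray actor that keeps its box area stocked with a random skill ball.
; A two-second looping timer, also run on BeginPlay, checks the box for overlapping WorldDynamic or PhysicsBody actors.
; When empty, it picks a random name from its list, looks up DT_SkillBall and spawns that class.
; It passes rotation, energy cost and split count to the ball through BPI_SkillBallInterface.
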(event Custom|CheckSkillBallInBox
  (bind _randomskillballnamelist (Variables|Default|GetRandomSkillBallNameList))
  (bind _box (Variables|Default|GetBox))
  (bind _outactors (Class|KismetSystemLibrary|BoxOverlapActorsNEW (Transformation|GetWorldLocation _box) (Variables|/Script/Engine.BoxComponent|GetBoxExtent _box) (Utilities|Array|MakeArray "ObjectTypeQuery2" "ObjectTypeQuery4")))
  (if (== (Utilities|Array|Length _outactors) 0)
    (bind _returnvalue (Utilities|GetDataTableRow "/Game/ClashRoyaleTest/Blueprints/GameDesign/DT_SkillBall.DT_SkillBall" (Utilities|String|StringToName (Utilities|Array|Get(acopy) _randomskillballnamelist (Math|Random|RandomIntegerinRange 0 (Utilities|Array|LastIndex _randomskillballnamelist)))))
      (:then
        (bind _returnvalue_2 (Game|SpawnActorfromClass (.Class (Utilities|Struct|BreakS_SkillBallDataTable _returnvalue)) (Math|Transform|MakeTransform (Transformation|GetWorldLocation (Variables|Default|GetBox)) (Transformation|GetWorldRotation (Variables|Default|GetArrow)) "1,1,1") "Undefined" 0 0))
        (if (Utilities|DoesObjectImplementInterface _returnvalue_2 "/Game/ClashRoyaleTest/Blueprints/SkillBall/BPI_SkillBallInterface.BPI_SkillBallInterface_C")
          (Class|BPISkillBallInterface|SetSkillBallRotation(Message) _returnvalue_2 (Transformation|GetWorldRotation (Variables|Default|GetArrow)))
          (Class|BPISkillBallInterface|SetSkillBallEnergyCost(Message) _returnvalue_2 (.EnergyCost (Utilities|Struct|BreakS_SkillBallDataTable _returnvalue)))
          (Class|BPISkillBallInterface|SetSkillBallSplitCount(Message) _returnvalue_2 (.SpawnSoldiersCount (Utilities|Struct|BreakS_SkillBallDataTable _returnvalue))))))))

(event EventBeginPlay
  (Utilities|Time|SetTimerbyEvent (delegate Custom|CheckSkillBallInBox) 2.0 true)
  (CallFunction|CheckSkillBallinBox))

(fn ConstructionScript)