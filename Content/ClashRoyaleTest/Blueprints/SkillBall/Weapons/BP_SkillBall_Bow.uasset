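; VR bow weapon that starts as an energy-priced skill ball and becomes a bow on first pickup.
; The second hand drags the string, stretching two scaled meshes and spawning single or multi-shot arrows.
; Release launches them at pull-scaled speed and decrements ammo while a timeline resets the string.
; Easy mode attaches the bow without dropping and destroys it when empty; complex mode allows physics drops, using extreme damping while held.
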(event Custom|UpdateString
  (params (CenterPosition :type Vector))
  (bind _returnvalue (* 1.0 0.003))
  (bind _end2 (Variables|Default|Getend2))
  (bind _end1 (Variables|Default|Getend1))
  (bind _returnvalue_2 (Transformation|GetWorldLocation _end2))
  (bind _returnvalue_3 (Transformation|GetWorldLocation _end1))
  (Utilities|FlowControl|Sequence
    (:then_0
      ;[1 1 1] update the string
      (Transformation|SetWorldTransform (Variables|Default|Getstring2) (Math|Transform|MakeTransform (* (+ CenterPosition _returnvalue_2) 0.5) (Math|Rotator|FindLookatRotation CenterPosition _returnvalue_2) (Math|Vector|MakeVector (* (Math|Vector|VectorLength (- CenterPosition _returnvalue_2)) 0.01) _returnvalue _returnvalue)) false false)
      (Transformation|SetWorldTransform (Variables|Default|Getstring1) (Math|Transform|MakeTransform (* (+ CenterPosition _returnvalue_3) 0.5) (Math|Rotator|FindLookatRotation CenterPosition _returnvalue_3) (Math|Vector|MakeVector (* (Math|Vector|VectorLength (- CenterPosition _returnvalue_3)) 0.01) _returnvalue _returnvalue)) false false))
    (:then_1
      ;[1 1 1] update the arrow
      (if (> (Math|Vector|VectorLength (- CenterPosition (* (+ (Transformation|GetWorldLocation (Variables|Default|Getend1)) (Transformation|GetWorldLocation (Variables|Default|Getend2))) 0.5))) 15.0)
        (Utilities|FlowControl|DoOnce false
          (:Completed
            (CallFunction|SpawnArrow CenterPosition)))))
    (:then_2
      (CallFunction|UpdateArrow CenterPosition))))

(event Custom|ResetArrowSpawn
  ;[1 1 1] update the arrow
  (Utilities|FlowControl|DoOnce false) ; enters at Reset
)

(event Custom|UpdateArrow
  (params (HandPosition :type Vector))
  (bind _spawnedarrows (Variables|Default|GetSpawnedArrows))
  ;[1 1 1] arrow
  (if (Variables|NotUsed|GetNextShotIsMultiShot)
    (if (> (Utilities|Array|Length (Variables|Default|GetSpawnedArrows)) 0)
      (for (_array_element _array_index) (Variables|NotUsed|GetMutliShotXOffset)
        (Transformation|SetActorTransform (Utilities|Array|Get(acopy) (Variables|Default|GetSpawnedArrows) _array_index) (Math|Transform|MakeTransform HandPosition (Math|Rotator|FindLookatRotation HandPosition (Math|Transform|TransformLocation (Transformation|GetActorTransform) (Math|Vector|MakeVector _array_element 0.0 0.0))) "2.000000,2.000000,2.000000"))))
    (elif (> (Utilities|Array|Length _spawnedarrows) 0)
      (Transformation|SetActorTransform (Utilities|Array|Get(acopy) _spawnedarrows) (Math|Transform|MakeTransform HandPosition (Math|Rotator|FindLookatRotation HandPosition (Transformation|GetWorldLocation (Variables|Default|GetArrowAttatchPoint))) "2.000000,2.000000,2.000000")))))

(event Custom|PickupPressed
  ;[1 1 1] easy operate mode,bow attach to hand auto,no hand swap
)

(event Custom|ReleaseString
  (params (ReleasePosition :type Vector))
  (bind _inputconsumer (Variables|Default|GetInputConsumer))
  (Utilities|FlowControl|Sequence
    (:then_0
      ;[1 1 1] shoot arrow if have
      (Variables|NotUsed|SetNextShotIsMultiShot false)
      (for _array_element (Variables|Default|GetSpawnedArrows)
        (Transformation|DetachFromActor _array_element "KeepWorld" "KeepWorld" "KeepWorld")
        (Variables|/Script/Engine.MovementComponent|SetVelocity (Variables|/Game/ClashRoyaleTest/Blueprints/SpawnObject/Bullet/WeaponBullet/BP_Bow_Bullet.BP_Bow_Bullet_C|GetProjectileMovement _array_element) (* (Math|Vector|GetForwardVector (Variables|/Game/ClashRoyaleTest/Blueprints/SpawnObject/Bullet/WeaponBullet/BP_Bow_Bullet.BP_Bow_Bullet_C|GetStaticMesh _array_element)) (Math|Vector|VectorLength (* (- (* (+ (Transformation|GetWorldLocation (Variables|Default|Getend1)) (Transformation|GetWorldLocation (Variables|Default|Getend2))) 0.5) ReleasePosition) 5e+01))))
        (Components|Activation|SetActive (Variables|/Game/ClashRoyaleTest/Blueprints/SpawnObject/Bullet/WeaponBullet/BP_Bow_Bullet.BP_Bow_Bullet_C|GetProjectileMovement _array_element) true false)
        (Actor|SetLifeSpan _array_element 5.0)
        (Default|SetCollisionEnableDelay _array_element)
        (Collision|IgnoreActorwhenMoving (Variables|/Game/ClashRoyaleTest/Blueprints/SpawnObject/Bullet/WeaponBullet/BP_Bow_Bullet.BP_Bow_Bullet_C|GetStaticMesh _array_element) (Components|GetOwner self) true)
        (bind _outactors (Actor|GetAllActorsOfClass "/Game/ClashRoyaleTest/Blueprints/SpawnObject/Bullet/WeaponBullet/BP_Bow_Bullet.BP_Bow_Bullet_C"))
        (for _array_element_2 _outactors
          (Collision|IgnoreActorwhenMoving (Variables|/Game/ClashRoyaleTest/Blueprints/SpawnObject/Bullet/WeaponBullet/BP_Bow_Bullet.BP_Bow_Bullet_C|GetStaticMesh _array_element) _array_element_2 true))
        (bind _result (Math|Integer|DecrementInt (Variables|Default|GetBulletCount))
          (:%20%20
            (Rendering|Components|TextRender|SetText (Variables|Default|GetBulletCountText) (Utilities|Text|ToText(Integer) _result))
            (if (Variables|/Game/ClashRoyaleTest/Blueprints/GameModeEtc/BP_GameInstance.BP_GameInstance_C|GetIsEasyOperateMode (.AsBP%20Game%20Instance (Utilities|Casting|CastToBP_GameInstance (Game|GetGameInstance))))
              (if (== _result 0)
                (Utilities|IsValid _inputconsumer
                  (:Is%20Valid
                    (Actor|DestroyActor _inputconsumer))
                  (:Is%20Not%20Valid
                    _))
                (Actor|DestroyActor))))))
      (Utilities|Array|Clear (Variables|Default|GetSpawnedArrows)))
    (:then_1
      ;[1 1 1] update string
      (bind _lerp (Timeline|ReleaseStringTimeLine PlayFromStart)
        (:Update
          (CallFunction|UpdateString (Math|Vector|Lerp(Vector) ReleasePosition (* (+ (Transformation|GetWorldLocation (Variables|Default|Getend1)) (Transformation|GetWorldLocation (Variables|Default|Getend2))) 0.5) _lerp)))
        (:Finished
          (CallFunction|ResetArrowSpawn))))))

(event Custom|SpawnArrow
  (params (HandPosition :type Vector))
  ;[1 1 1] arrow
  (if (> (Variables|Default|GetBulletCount) 0)
    (if (Variables|NotUsed|GetNextShotIsMultiShot)
      (for _array_element (Variables|NotUsed|GetMutliShotXOffset)
        (bind _returnvalue (Game|SpawnActorfromClass "/Game/ClashRoyaleTest/Blueprints/SpawnObject/Bullet/WeaponBullet/BP_Bow_Bullet.BP_Bow_Bullet_C" (Math|Transform|MakeTransform HandPosition (Math|Rotator|FindLookatRotation HandPosition (Math|Transform|TransformLocation (Transformation|GetActorTransform) (Math|Vector|MakeVector _array_element 0.0 0.0))) "2.000000,2.000000,2.000000") "Undefined" (.AsPawn (Utilities|Casting|CastToPawn (Components|GetOwner self))) (Variables|/Game/ClashRoyaleTest/Blueprints/GameModeEtc/BP_BattleField_PlayerController.BP_BattleField_PlayerController_C|GetCamp (.AsBP%20Battle%20Field%20Player%20Controller (Utilities|Casting|CastToBP_BattleField_PlayerController (Game|GetPlayerController 0)))) 0))
        (Actor|SetLifeSpan 0.0)
        (Collision|IgnoreActorwhenMoving (Variables|/Game/ClashRoyaleTest/Blueprints/SpawnObject/Bullet/WeaponBullet/BP_Bow_Bullet.BP_Bow_Bullet_C|GetStaticMesh _returnvalue) self true)
        (Utilities|Array|Add (Variables|Default|GetSpawnedArrows) _returnvalue))
      (else
        (bind _returnvalue_2 (Game|SpawnActorfromClass "/Game/ClashRoyaleTest/Blueprints/SpawnObject/Bullet/WeaponBullet/BP_Bow_Bullet.BP_Bow_Bullet_C" (Math|Transform|MakeTransform HandPosition (Math|Rotator|FindLookatRotation HandPosition (Transformation|GetWorldLocation (Variables|Default|GetArrowAttatchPoint))) "2.000000,2.000000,2.000000") "Undefined" (.AsPawn (Utilities|Casting|CastToPawn (Components|GetOwner self))) (Variables|/Game/ClashRoyaleTest/Blueprints/GameModeEtc/BP_BattleField_PlayerController.BP_BattleField_PlayerController_C|GetCamp (.AsBP%20Battle%20Field%20Player%20Controller (Utilities|Casting|CastToBP_BattleField_PlayerController (Game|GetPlayerController 0)))) 0))
        (Actor|SetLifeSpan 0.0)
        (Collision|IgnoreActorwhenMoving (Variables|/Game/ClashRoyaleTest/Blueprints/SpawnObject/Bullet/WeaponBullet/BP_Bow_Bullet.BP_Bow_Bullet_C|GetStaticMesh _returnvalue_2) self true)
        (Utilities|Array|Add (Variables|Default|GetSpawnedArrows) _returnvalue_2)))))

(event Collision|EventHit
  (params (MyComp :type Primitive%20Component%20Object%20Reference) (Other :type Actor%20Object%20Reference) (OtherComp :type Primitive%20Component%20Object%20Reference) (bSelfMoved :type Boolean) (HitLocation :type Vector) (HitNormal :type Vector :default "0, 0, 0") (NormalImpulse :type Vector :default "0, 0, 0") (Hit :type Hit%20Result%20Structure%20%28by%20ref%29))
  (if (Utilities|Enum|Equal(Enum) (Utilities|String|ToString(Name) (Utilities|Array|Get(acopy) (Variables|/Script/Engine.Actor|GetTags Other))) "Floor")
    (Utilities|FlowControl|DoOnce false
      (:Completed
        (Actor|SetLifeSpan 2.0)))))

(event EventOnPickup
  (params (Interactor :type World%20Interactor%20Object%20Reference))
  (bind _returnvalue (Math|Transform|MakeTransform "0, 0, 0"))
  (bind _bowmesh (Variables|Default|GetBowMesh))
  (bind _bowmesh_2 (Variables|Default|GetBowMesh))
  (bind _currentinteractor (Variables|Default|GetCurrentInteractor))
  (if (not (Variables|Default|GetIsPickuped))
    (Variables|Default|SetIsPickuped true)
    (Variables|Default|SetPickupInteractor Interactor)
    (Utilities|FlowControl|Sequence
      (:then_0
        ;[1 1 1] something do once at first pick up
        (Utilities|FlowControl|DoOnce false
          (:Completed
            ;;[1 1 1] see construction
            (Collision|SetCollisionEnabled (Variables|Default|GetBowMesh) "QueryAndPhysics")
            ;;[1 1 1] hide skill ball,show bow
            (Development|SetHiddeninGame (Variables|Default|GetParticleSystem) true false)
            (Development|SetHiddeninGame (Variables|Default|GetBowMesh) false false)
            ;;[1 1 1] energy consume
            (Default|ConsumeEnergy (.AsBP%20Battle%20Field%20Player%20Controller (Utilities|Casting|CastToBP_BattleField_PlayerController (Game|GetPlayerController 0))) (Math|Conversions|ToFloat(Integer) (Variables|Default|GetEnergyCost)))
            (Development|SetHiddeninGame (Variables|Default|GetEnergyCostText) true false))))
      (:then_1
        (if (Variables|/Game/ClashRoyaleTest/Blueprints/GameModeEtc/BP_GameInstance.BP_GameInstance_C|GetIsEasyOperateMode (.AsBP%20Game%20Instance (Utilities|Casting|CastToBP_GameInstance (Game|GetGameInstance))))
          ;[1 1 1] easy operate mode,bow attach to hand auto,no hand swap
          (Physics|SetSimulatePhysics (Variables|Default|GetBowMesh) false)
          (Collision|SetCollisionEnabled (Variables|Default|GetBowMesh) "NoCollision")
          (Utilities|IsValid _currentinteractor
            (:Is%20Valid
              (switch Utilities|FlowControl|Switch|SwitchonEControllerHand (Default|GetHand _currentinteractor)
                (:Left
                  (bind _returnvalue_2 (Game|SpawnActorfromClass "/Game/ExampleContent/VR_World_Interaction/Blueprints/HelperObjects/LeftPickupInputConsumer.LeftPickupInputConsumer_C" _returnvalue "Undefined" 0 0))
                  (bind _output_get (Variables|Default|SetInputConsumer _returnvalue_2))
                  (EventDispatchers|AssignInputPressed _output_get (delegate Custom|PickupPressed)))
                (:Right
                  (bind _returnvalue_3 (Game|SpawnActorfromClass "/Game/ExampleContent/VR_World_Interaction/Blueprints/HelperObjects/RightPickupInputConsumer.RightPickupInputConsumer_C" _returnvalue "Undefined" 0 0))
                  (bind _output_get_2 (Variables|Default|SetInputConsumer _returnvalue_3))
                  (EventDispatchers|AssignInputPressed _output_get_2 (delegate Custom|PickupPressed))))
              (Variables|Default|SetIsCanPickup false)))
          (else
            ;[1 1 1] complex operate mode,use physics
            (Class|PrimitiveComponent|SetLinearDamping _bowmesh 0.01)
            (Class|PrimitiveComponent|SetAngularDamping _bowmesh 0.0)
            (Physics|SetEnableGravity _bowmesh_2 false)
            (Variables|Default|SetPreviousLinearDamping (Class|PrimitiveComponent|GetLinearDamping _bowmesh_2))
            (Variables|Default|SetPreviousAngularDamping (Class|PrimitiveComponent|GetAngularDamping _bowmesh_2))
            (Class|PrimitiveComponent|SetLinearDamping _bowmesh_2 9999999999.0)
            (Class|PrimitiveComponent|SetAngularDamping _bowmesh_2 99999999.0)))))))

(event EventTick
  (params (DeltaSeconds :type Float%20%28single-precision%29))
  (bind _particlesystem (Variables|Default|GetParticleSystem))
  ;[1 1 1] energy
  (if (not (Variables|Default|GetIsPickuped))
    (if (> (Math|Conversions|ToFloat(Integer) (Variables|Default|GetEnergyCost)) (Variables|/Game/ClashRoyaleTest/Blueprints/GameModeEtc/BP_BattleField_PlayerController.BP_BattleField_PlayerController_C|GetCurEnergy (.AsBP%20Battle%20Field%20Player%20Controller (Utilities|Casting|CastToBP_BattleField_PlayerController (Game|GetPlayerController 0)))))
      (Utilities|FlowControl|DoOnce false :!label _label
        (:Completed
          (Variables|Default|SetIsCanPickup false)
          (bind _output_get (Variables|Default|SetTextColor "(R=1.000000,G=0.000000,B=0.000000,A=1.000000)"))
          (Rendering|Components|TextRender|SetTextRenderColor (Variables|Default|GetEnergyCostText) (Math|Conversions|ToColor(LinearColor) _output_get))
          (Effects|Components|ParticleSystem|SetFloatParameter _particlesystem "Alpha" 0.8)
          (goto _label_2 Reset)))
      (else
        (Utilities|FlowControl|DoOnce false :!label _label_2
          (:Completed
            (Variables|Default|SetIsCanPickup true)
            (bind _output_get_2 (Variables|Default|SetTextColor "(R=0.000000,G=0.000000,B=1.000000,A=1.000000)"))
            (Rendering|Components|TextRender|SetTextRenderColor (Variables|Default|GetEnergyCostText) (Math|Conversions|ToColor(LinearColor) _output_get_2))
            (Effects|Components|ParticleSystem|SetFloatParameter _particlesystem "Alpha" 0.0)
            (goto _label Reset)))))))

(event EventSetSkillBallEnergyCost
  (params (EnergyCost :type Integer))
  ;[1 1 1] energy
  (Variables|Default|SetEnergyCost EnergyCost)
  (Rendering|Components|TextRender|SetText (Variables|Default|GetEnergyCostText) (Utilities|Text|ToText(Integer) (Variables|Default|GetEnergyCost))))

(event EventOnDrag
  (params (Interactor :type World%20Interactor%20Object%20Reference))
  ;[1 1 1] pickup hand is not drag hand
  (if (!= Interactor (Variables|Default|GetPickupInteractor))
    (if (Variables|Default|GetIsPulling)
      (CallFunction|UpdateString (Transformation|GetWorldLocation Interactor)))))

(event EventOnHover
  (params (Interactor :type World%20Interactor%20Object%20Reference))
  (Variables|Default|SetCurrentInteractor Interactor))

(event EventOnDragEnd
  (params (Interactor :type World%20Interactor%20Object%20Reference))
  ;[1 1 1] pickup hand is not drag hand
  (if (!= Interactor (Variables|Default|GetPickupInteractor))
    (if (Variables|Default|GetIsPulling)
      (CallFunction|ReleaseString (Transformation|GetWorldLocation Interactor))
      (Variables|Default|SetIsPulling false))))

(event EventOnDrop
  (params (Velocity :type Vector) (AngularVelocity :type Vector) (Interactor :type World%20Interactor%20Object%20Reference))
  (bind _bowmesh (Variables|Default|GetBowMesh))
  (if (not (Variables|/Game/ClashRoyaleTest/Blueprints/GameModeEtc/BP_GameInstance.BP_GameInstance_C|GetIsEasyOperateMode (.AsBP%20Game%20Instance (Utilities|Casting|CastToBP_GameInstance (Game|GetGameInstance)))))
    ;[1 1 1] complex operate mode
    (Variables|Default|SetIsPickuped false)
    (Class|PrimitiveComponent|SetLinearDamping _bowmesh (Variables|Default|GetPreviousLinearDamping))
    (Class|PrimitiveComponent|SetAngularDamping _bowmesh (Variables|Default|GetPreviousAngularDamping))
    (Physics|SetEnableGravity _bowmesh true)
    (Physics|AddImpulse _bowmesh Velocity "None" true)
    (Class|PrimitiveComponent|AddAngularImpulse _bowmesh AngularVelocity "None" true)))

(event EventOnDragStart
  (params (Interactor :type World%20Interactor%20Object%20Reference))
  ;[1 1 1] pickup hand is not drag hand
  (if (!= Interactor (Variables|Default|GetPickupInteractor))
    (if (Variables|Default|GetIsPickuped)
      (bind _outcomponents (Class|KismetSystemLibrary|SphereOverlapComponentsNEW (Transformation|GetWorldLocation Interactor) 1e+01 (Utilities|Array|MakeArray "ObjectTypeQuery2") "/Script/Engine.SphereComponent"))
      (if (> (Utilities|Array|Length _outcomponents) 0)
        (if (Components|ComponentHasTag (Utilities|Array|Get(acopy) _outcomponents) "Emitter")
          (Variables|Default|SetIsPulling true))))))

(fn ConstructionScript
  (bind _bowmesh (Variables|Default|GetBowMesh))
  (Utilities|FlowControl|Sequence
    (:then_0
      ;[1 1 1] set text
      (Rendering|Components|TextRender|SetText (Variables|Default|GetEnergyCostText) (Utilities|Text|ToText(Integer) (Variables|Default|GetEnergyCost)))
      (Rendering|Components|TextRender|SetText (Variables|Default|GetBulletCountText) (Utilities|Text|ToText(Integer) (Variables|Default|GetBulletCount))))
    (:then_1
      ;[1 1 1] set string init position
      (CallFunction|UpdateString (* (+ (Transformation|GetWorldLocation (Variables|Default|Getend1)) (Transformation|GetWorldLocation (Variables|Default|Getend2))) 0.5)))
    (:then_2
      ;[1 1 1] set physics
      (Class|PrimitiveComponent|SetLinearDamping _bowmesh 9999999999.0)
      (Class|PrimitiveComponent|SetAngularDamping _bowmesh 99999999.0))
    (:then_3
      ;[1 1 1] set hidden
      (Development|SetHiddeninGame (Variables|Default|GetBowMesh) true false)
      (Development|SetHiddeninGame (Variables|Default|GetParticleSystem) false false))
    (:then_4
      ;[1 1 1] 修复玩家可以在球外面抓起弓的bug
      (Collision|SetCollisionEnabled (Variables|Default|GetBowMesh) "NoCollision"))))

(fn CanDrop
  (return (not (Variables|/Game/ClashRoyaleTest/Blueprints/GameModeEtc/BP_GameInstance.BP_GameInstance_C|GetIsEasyOperateMode (.AsBP%20Game%20Instance (Utilities|Casting|CastToBP_GameInstance (Game|GetGameInstance)))))))

(fn CanPickup
  (return (Variables|Default|GetIsCanPickup)))

(fn GetAttachLocation
  (return "3.923019,0.000114,-19.554785"))

(fn GetAttachRotation
  (return "0,180.000000,-180.000000"))

(fn ShouldSnaptoInteractor
  (return true))