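; A VR skill ball that turns into a limited-ammo pistol when picked up, spending the player's energy.
; Tick compares energy to cost to drive pickup availability, text color and particle alpha; first pickup swaps the particle for the mesh, and use spawns camp-tagged bullets.
; Easy mode blocks dropping, spawns hand-specific input consumers and destroys the empty gun.
; Complex mode allows physics throws via damping and gravity toggles, with floor hits starting timed destruction.
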(event Custom|PickupPressed
  ;[1 1 1] easy operate mode,pistol attach to hand auto,no hand swap
  (Default|UseHoveredObject (Variables|Default|GetCurrentInteractor)))

(event Collision|EventHit
  (params (MyComp :type Primitive%20Component%20Object%20Reference) (Other :type Actor%20Object%20Reference) (OtherComp :type Primitive%20Component%20Object%20Reference) (bSelfMoved :type Boolean) (HitLocation :type Vector) (HitNormal :type Vector :default "0, 0, 0") (NormalImpulse :type Vector :default "0, 0, 0") (Hit :type Hit%20Result%20Structure%20%28by%20ref%29))
  ;[1 1 1] drop on floor will destroy
  (if (Utilities|Enum|Equal(Enum) (Utilities|String|ToString(Name) (Utilities|Array|Get(acopy) (Variables|/Script/Engine.Actor|GetTags Other))) "Floor")
    (Utilities|FlowControl|DoOnce false
      (:Completed
        (Actor|SetLifeSpan 2.0)))))

(event EventOnPickup
  (params (Interactor :type World%20Interactor%20Object%20Reference))
  (bind _returnvalue (Math|Transform|MakeTransform "0, 0, 0"))
  (bind _pistolmesh (Variables|Default|GetPistolMesh))
  (bind _pistolmesh_2 (Variables|Default|GetPistolMesh))
  (bind _currentinteractor (Variables|Default|GetCurrentInteractor))
  (if (not (Variables|Default|GetIsPickuped))
    (Variables|Default|SetIsPickuped true)
    (Utilities|FlowControl|Sequence
      (:then_0
        ;[1 1 1] something do once at first pick up
        (Utilities|FlowControl|DoOnce false
          (:Completed
            ;;[1 1 1] hide skill ball,show pistol
            (Development|SetHiddeninGame (Variables|Default|GetPistolMesh) false false)
            (Development|SetHiddeninGame (Variables|Default|GetParticleSystem) true false)
            ;;[1 1 1] energy consume
            (Default|ConsumeEnergy (.AsBP%20Battle%20Field%20Player%20Controller (Utilities|Casting|CastToBP_BattleField_PlayerController (Game|GetPlayerController 0))) (Math|Conversions|ToFloat(Integer) (Variables|Default|GetEnergyCost)))
            (Development|SetHiddeninGame (Variables|Default|GetEnergyCostText) true false))))
      (:then_1
        (if (Variables|/Game/ClashRoyaleTest/Blueprints/GameModeEtc/BP_GameInstance.BP_GameInstance_C|GetIsEasyOperateMode (.AsBP%20Game%20Instance (Utilities|Casting|CastToBP_GameInstance (Game|GetGameInstance))))
          ;[1 1 1] easy operate mode,pistol attach to hand auto,no hand swap
          (Physics|SetSimulatePhysics (Variables|Default|GetPistolMesh) false)
          (Utilities|IsValid _currentinteractor
            (:Is%20Valid
              (switch Utilities|FlowControl|Switch|SwitchonEControllerHand (Default|GetHand _currentinteractor)
                (:Left
                  (bind _returnvalue_2 (Game|SpawnActorfromClass "/Game/ExampleContent/VR_World_Interaction/Blueprints/HelperObjects/LeftPickupInputConsumer.LeftPickupInputConsumer_C" _returnvalue "Undefined" 0 0))
                  (bind _output_get (Variables|Default|SetInputConsumer _returnvalue_2))
                  (EventDispatchers|AssignInputPressed _output_get (delegate Custom|PickupPressed)))
                (:Right
                  (bind _returnvalue_3 (Game|SpawnActorfromClass "/Game/ExampleContent/VR_World_Interaction/Blueprints/HelperObjects/RightPickupInputConsumer.RightPickupInputConsumer_C" _returnvalue "Undefined" 0 0))
                  (bind _output_get_2 (Variables|Default|SetInputConsumer _returnvalue_3))
                  (EventDispatchers|AssignInputPressed _output_get_2 (delegate Custom|PickupPressed))))
              (Variables|Default|SetIsCanPickup false)))
          (else
            ;[1 1 1] complex operate mode,use physics,can do hand swap
            (Class|PrimitiveComponent|SetLinearDamping _pistolmesh 0.01)
            (Class|PrimitiveComponent|SetAngularDamping _pistolmesh 0.0)
            (Physics|SetEnableGravity _pistolmesh_2 false)
            (Variables|Default|SetPreviousLinearDamping (Class|PrimitiveComponent|GetLinearDamping _pistolmesh_2))
            (Variables|Default|SetPreviousAngularDamping (Class|PrimitiveComponent|GetAngularDamping _pistolmesh_2))
            (Class|PrimitiveComponent|SetLinearDamping _pistolmesh_2 9999999999.0)
            (Class|PrimitiveComponent|SetAngularDamping _pistolmesh_2 99999999.0)))))))

(event EventTick
  (params (DeltaSeconds :type Float%20%28single-precision%29))
  (bind _particlesystem (Variables|Default|GetParticleSystem))
  ;[1 1 1] energy cost text deal
  (if (not (Variables|Default|GetIsPickuped))
    (if (> (Math|Conversions|ToFloat(Integer) (Variables|Default|GetEnergyCost)) (Variables|/Game/ClashRoyaleTest/Blueprints/GameModeEtc/BP_BattleField_PlayerController.BP_BattleField_PlayerController_C|GetCurEnergy (.AsBP%20Battle%20Field%20Player%20Controller (Utilities|Casting|CastToBP_BattleField_PlayerController (Game|GetPlayerController 0)))))
      (Utilities|FlowControl|DoOnce false :!label _label
        (:Completed
          (Variables|Default|SetIsCanPickup false)
          (bind _output_get (Variables|Default|SetTextColor "(R=1.000000,G=0.000000,B=0.000000,A=1.000000)"))
          (Rendering|Components|TextRender|SetTextRenderColor (Variables|Default|GetEnergyCostText) (Math|Conversions|ToColor(LinearColor) _output_get))
          (Effects|Components|ParticleSystem|SetFloatParameter _particlesystem "Alpha" 0.8)
          (goto _label_2 Reset)))
      (else
        (Utilities|FlowControl|DoOnce false :!label _label_2
          (:Completed
            (Variables|Default|SetIsCanPickup true)
            (bind _output_get_2 (Variables|Default|SetTextColor "(R=0.000000,G=0.000000,B=1.000000,A=1.000000)"))
            (Rendering|Components|TextRender|SetTextRenderColor (Variables|Default|GetEnergyCostText) (Math|Conversions|ToColor(LinearColor) _output_get_2))
            (Effects|Components|ParticleSystem|SetFloatParameter _particlesystem "Alpha" 0.0)
            (goto _label Reset)))))))

(event EventSetSkillBallEnergyCost
  (params (EnergyCost :type Integer))
  ;[1 1 1] energy cost text deal
  (Variables|Default|SetEnergyCost EnergyCost)
  (Rendering|Components|TextRender|SetText (Variables|Default|GetEnergyCostText) (Utilities|Text|ToText(Integer) (Variables|Default|GetEnergyCost))))

(event EventOnHover
  (params (Interactor :type World%20Interactor%20Object%20Reference))
  (Variables|Default|SetCurrentInteractor Interactor))

(event EventOnDrop
  (params (Velocity :type Vector) (AngularVelocity :type Vector) (Interactor :type World%20Interactor%20Object%20Reference))
  (bind _pistolmesh (Variables|Default|GetPistolMesh))
  (if (not (Variables|/Game/ClashRoyaleTest/Blueprints/GameModeEtc/BP_GameInstance.BP_GameInstance_C|GetIsEasyOperateMode (.AsBP%20Game%20Instance (Utilities|Casting|CastToBP_GameInstance (Game|GetGameInstance)))))
    ;[1 1 1] complex operate mode,use physics
    (Variables|Default|SetIsPickuped false)
    (Class|PrimitiveComponent|SetLinearDamping _pistolmesh (Variables|Default|GetPreviousLinearDamping))
    (Class|PrimitiveComponent|SetAngularDamping _pistolmesh (Variables|Default|GetPreviousAngularDamping))
    (Physics|SetEnableGravity _pistolmesh true)
    (Physics|AddImpulse _pistolmesh Velocity "None" true)
    (Class|PrimitiveComponent|AddAngularImpulse _pistolmesh AngularVelocity "None" true)))

(event EventOnUse
  (bind _arrow (Variables|Default|GetArrow))
  (bind _inputconsumer (Variables|Default|GetInputConsumer))
  ;[1 1 1] fire
  (if (Variables|Default|GetIsPickuped)
    (if (> (Variables|Default|GetBulletCount) 0)
      (Game|SpawnActorfromClass "/Game/ClashRoyaleTest/Blueprints/SpawnObject/Bullet/WeaponBullet/BP_PistolBullet.BP_PistolBullet_C" (Math|Transform|MakeTransform (Transformation|GetWorldLocation _arrow) (Transformation|GetWorldRotation _arrow) "1,1,1") "Undefined" 0 (Variables|/Game/ClashRoyaleTest/Blueprints/GameModeEtc/BP_BattleField_PlayerController.BP_BattleField_PlayerController_C|GetCamp (.AsBP%20Battle%20Field%20Player%20Controller (Utilities|Casting|CastToBP_BattleField_PlayerController (Game|GetPlayerController 0)))) 0)
      (bind _result (Math|Integer|DecrementInt (Variables|Default|GetBulletCount))
        (:%20%20
          (Rendering|Components|TextRender|SetText (Variables|Default|GetBulletCountText) (Utilities|Text|ToText(Integer) _result))
          ;[1 1 1] easy operate mode,pistol auto destory after bullet is zero
          (if (Variables|/Game/ClashRoyaleTest/Blueprints/GameModeEtc/BP_GameInstance.BP_GameInstance_C|GetIsEasyOperateMode (.AsBP%20Game%20Instance (Utilities|Casting|CastToBP_GameInstance (Game|GetGameInstance))))
            (if (== _result 0)
              (Utilities|IsValid _inputconsumer
                (:Is%20Valid
                  (Actor|DestroyActor _inputconsumer))
                (:Is%20Not%20Valid
                  _))
              (Actor|DestroyActor))))))))

(fn ConstructionScript
  (bind _pistolmesh (Variables|Default|GetPistolMesh))
  ;[1 1 1] set text
  (Rendering|Components|TextRender|SetText (Variables|Default|GetEnergyCostText) (Utilities|Text|ToText(Integer) (Variables|Default|GetEnergyCost)))
  (Rendering|Components|TextRender|SetText (Variables|Default|GetBulletCountText) (Utilities|Text|ToText(Integer) (Variables|Default|GetBulletCount)))
  ;[1 1 1] set physics
  (Class|PrimitiveComponent|SetLinearDamping _pistolmesh 9999999999.0)
  (Class|PrimitiveComponent|SetAngularDamping _pistolmesh 99999999.0)
  ;[1 1 1] set hidden
  (Development|SetHiddeninGame (Variables|Default|GetPistolMesh) true false))

(fn CanDrop
  (return (not (Variables|/Game/ClashRoyaleTest/Blueprints/GameModeEtc/BP_GameInstance.BP_GameInstance_C|GetIsEasyOperateMode (.AsBP%20Game%20Instance (Utilities|Casting|CastToBP_GameInstance (Game|GetGameInstance)))))))

(fn CanPickup
  (return (Variables|Default|GetIsCanPickup)))

(fn GetAttachLocation
  (return "10.353254, 0,0.914016"))

(fn GetAttachRotation
  (return "55.000000, 0, 0"))

(fn ShouldSnaptoInteractor
  (return true))