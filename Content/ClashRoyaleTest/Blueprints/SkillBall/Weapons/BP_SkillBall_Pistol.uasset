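; BP_SkillBall_Pistol is an interactable skill ball pickup that turns into a pistol when picked up.
; On hover it stores the interactor; on pickup it spawns BP_Pistol at its location, destroys itself, then calls Pickup on that stored interactor.
; Its attach location and rotation functions return zero, and it does not snap to the interactor.
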(event EventOnPickup
  (Game|SpawnActorfromClass "/Game/ClashRoyaleTest/Blueprints/SpawnObject/Weapons/BP_Pistol.BP_Pistol_C" (Math|Transform|MakeTransform (Transformation|GetActorLocation) "0, 0, 0" "1,1,1") "Undefined" 0 0)
  (Actor|DestroyActor)
  (Default|Pickup (Variables|Default|GetCurrentIteractor)))

(event EventOnHover
  (params (Interactor :type World%20Interactor%20Object%20Reference))
  (Variables|Default|SetCurrentIteractor Interactor))

(fn ConstructionScript)

(fn GetAttachLocation
  (return "0, 0, 0"))

(fn GetAttachRotation
  (return "0, 0, 0"))

(fn ShouldSnaptoInteractor
  (return false))