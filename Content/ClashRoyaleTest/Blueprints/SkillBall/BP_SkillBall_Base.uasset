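; Base skill ball actor that is picked up for an energy cost and thrown through projectile movement.
; Tick compares its cost with player 0's energy, toggling pickup permission, text color and particle alpha.
; First pickup consumes energy and hides the cost text; dropping launches it at boosted velocity with a limited lifespan.
; Split counts above one precompute evenly spaced radial vectors, and an older physics-based hold/throw approach remains unwired.
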(event EventTick
  (params (DeltaSeconds :type Float%20%28single-precision%29))
  (bind _particlesystem (Variables|Default|GetParticleSystem))
  (if (not (Variables|Default|GetIsPickuped))
    (if (> (Math|Conversions|ToFloat(Integer) (Variables|Default|GetEnergyCost)) (Variables|/Game/ClashRoyaleTest/Blueprints/GameModeEtc/BP_BattleField_PlayerController.BP_BattleField_PlayerController_C|GetCurEnergy (.AsBP%20Battle%20Field%20Player%20Controller (Utilities|Casting|CastToBP_BattleField_PlayerController (Game|GetPlayerController 0)))))
      (Utilities|FlowControl|DoOnce false :!label _label
        (:Completed
          (Variables|Default|SetIsCanPickup false)
          (bind _output_get (Variables|Default|SetTextColor "(R=1.000000,G=0.000000,B=0.000000,A=1.000000)"))
          (Rendering|Components|TextRender|SetTextRenderColor (Variables|Default|GetEnergyCostText) (Math|Conversions|ToColor(LinearColor) _output_get))
          (Effects|Components|ParticleSystem|SetFloatParameter _particlesystem "Alpha" 0.8)
          (goto _label_2 Reset)))
      (else
        (Utilities|FlowControl|DoOnce false :!label _label_2
          (:Completed
            (Variables|Default|SetIsCanPickup true)
            (bind _output_get_2 (Variables|Default|SetTextColor "(R=0.000000,G=0.000000,B=1.000000,A=1.000000)"))
            (Rendering|Components|TextRender|SetTextRenderColor (Variables|Default|GetEnergyCostText) (Math|Conversions|ToColor(LinearColor) _output_get_2))
            (Effects|Components|ParticleSystem|SetFloatParameter _particlesystem "Alpha" 0.0)
            (goto _label Reset)))))))

(event EventOnDrop
  (params (Velocity :type Vector) (AngularVelocity :type Vector) (Interactor :type World%20Interactor%20Object%20Reference))
  ;[1 1 1] projectile method
  (Variables|/Script/Engine.MovementComponent|SetVelocity (Variables|Default|GetProjectileMovement) (* Velocity 1.6))
  (Components|Activation|SetActive (Variables|Default|GetProjectileMovement) true true)
  (Actor|SetLifeSpan 5.0))

(event EventSetSkillBallEnergyCost
  (params (EnergyCost :type Integer))
  (Variables|Default|SetEnergyCost EnergyCost)
  (Rendering|Components|TextRender|SetText (Variables|Default|GetEnergyCostText) (Utilities|Text|ToText(Integer) (Variables|Default|GetEnergyCost))))

(event EventOnPickup
  (params (Interactor :type World%20Interactor%20Object%20Reference))
  ;[1 1 1] projectile method
  (Components|Activation|SetActive (Variables|Default|GetProjectileMovement) false true)
  (Utilities|FlowControl|DoOnce false
    (:Completed
      (Default|ConsumeEnergy (.AsBP%20Battle%20Field%20Player%20Controller (Utilities|Casting|CastToBP_BattleField_PlayerController (Game|GetPlayerController 0))) (Math|Conversions|ToFloat(Integer) (Variables|Default|GetEnergyCost)))
      (Development|SetHiddeninGame (Variables|Default|GetEnergyCostText) true false)
      (Variables|Default|SetIsPickuped true))))

(event EventSetSkillBallSplitCount
  (params (SplitCount :type Integer))
  (bind _output_get (Variables|Default|SetSplitCount SplitCount))
  (if (> _output_get 1)
    (CallFunction|CalcSplitBallVector)))

(fn ConstructionScript
  (Rendering|Components|TextRender|SetText (Variables|Default|GetEnergyCostText) (Utilities|Text|ToText(Integer) (Variables|Default|GetEnergyCost))))

(fn CalcSplitBallVector
  (bind _output_get (LocalVariables|SetCurSplitBallCount (Variables|Default|GetSplitCount)))
  (LocalVariables|SetSplitAngular (Math|Conversions|ToFloat(Integer) (/ 360 (Variables|Default|GetSplitCount))))
  (while (> _output_get 0)
    (bind _result (Math|Integer|DecrementInt (LocalVariables|GetCurSplitBallCount))
      (:%20%20
        (Utilities|Array|Add (Variables|Default|GetRandomSplitBallVector) (Math|Vector|MakeVector (Math|Trig|Cos(Degrees) (* _result (LocalVariables|GetSplitAngular))) (Math|Trig|Sin(Degrees) (* _result (LocalVariables|GetSplitAngular))) 0.0))))))

(fn CanDrop
  (return true))

(fn CanPickup
  (return (Variables|Default|GetIsCanPickup)))

(fn GetAttachLocation
  (return "0, 0, 0"))

(fn GetAttachRotation
  (return "0, 0, 0"))

(fn ShouldSnaptoInteractor
  (return true))