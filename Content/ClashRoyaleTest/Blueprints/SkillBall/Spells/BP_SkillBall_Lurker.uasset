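; Lurker spell skill ball that erupts into a damaging ground-spike effect where it strikes the floor.
; The first hit on a Floor-tagged actor hides the ball's particles and shows a soil magic-circle emitter as a brief warning.
; After a delay it spawns the spikes, applies full radial damage with a camp-specific damage type, fires a radial impulse and destroys itself.
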(event Collision|EventHit
  (params (MyComp :type Primitive%20Component%20Object%20Reference) (Other :type Actor%20Object%20Reference) (OtherComp :type Primitive%20Component%20Object%20Reference) (bSelfMoved :type Boolean) (HitLocation :type Vector) (HitNormal :type Vector :default "0, 0, 0") (NormalImpulse :type Vector :default "0, 0, 0") (Hit :type Hit%20Result%20Structure%20%28by%20ref%29))
  (if (Utilities|Enum|Equal(Enum) (Utilities|String|ToString(Name) (Utilities|Array|Get(acopy) (Variables|/Script/Engine.Actor|GetTags Other))) "Floor")
    (Utilities|FlowControl|DoOnce false
      (:Completed
        (bind _output_get (Variables|Default|SetHitPosition HitLocation))
        (Development|SetHiddeninGame (Variables|Default|GetParticleSystem) true false)
        (bind _returnvalue (Effects|SpawnEmitteratLocation "/Game/ClashRoyaleTest/Effect/P_fazhen_soil.P_fazhen_soil" (Math|Vector|MakeVector (.X (Math|Vector|BreakVector _output_get)) (.Y (Math|Vector|BreakVector _output_get)) (+ (.Z (Math|Vector|BreakVector _output_get)) 1.0))))
        (Transformation|SetWorldScale3D _returnvalue "4.000000,4.000000,4.000000")
        (Utilities|FlowControl|Delay 1.0)
        (Components|DestroyComponent _returnvalue)
        (bind _returnvalue_2 (Effects|SpawnEmitteratLocation "/Game/ClashRoyaleTest/Effect/p_dici.P_dici" _output_get))
        (Transformation|SetWorldScale3D _returnvalue_2 "2.000000,2.000000,2.000000")
        (Game|Damage|ApplyRadialDamage 186.0 _output_get 1e+02 (Utilities|Select :Index (Variables|Default|GetCamp) :NewEnumerator0 "/Game/ClashRoyaleTest/Blueprints/CommonDefine/BP_CampDamageType_Blue.BP_CampDamageType_Blue_C" :NewEnumerator1 "/Game/ClashRoyaleTest/Blueprints/CommonDefine/BP_CampDamageType_Red.BP_CampDamageType_Red_C") 0 (Game|GetInstigator) 0 true "ECC_WorldDynamic")
        (if (Variables|Default|GetIsDebug)
          (Rendering|Debug|DrawDebugCircle (Variables|Default|GetHitPosition) 1e+02 12 "(R=1.000000,G=0.121217,B=0.071455,A=1.000000)" 5.0 1.0 "0.000000,1.000000,0.000000" "1.000000,0.000000,0.000000" true))
        (Class|RadialForceComponent|FireImpulse (Variables|Default|GetRadialForce))
        (Actor|DestroyActor)))))

(fn ConstructionScript
  (|CallParentFunction))