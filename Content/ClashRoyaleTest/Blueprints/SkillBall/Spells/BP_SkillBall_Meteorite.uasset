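; Meteorite spell skill ball that, on its first floor hit, calls down a meteorite dealing camp-specific radial damage along the stored skill rotation.
; A fire circle effect precedes the meteorite effect, then a delayed chain applies one heavy blast and three weaker ones stepping forward before destroying the actor.
; The first blast also fires a radial impulse and starts Tick sliding three more radial forces along local X, firing every frame.
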(event Collision|EventHit
  (params (MyComp :type Primitive%20Component%20Object%20Reference) (Other :type Actor%20Object%20Reference) (OtherComp :type Primitive%20Component%20Object%20Reference) (bSelfMoved :type Boolean) (HitLocation :type Vector) (HitNormal :type Vector :default "0, 0, 0") (NormalImpulse :type Vector :default "0, 0, 0") (Hit :type Hit%20Result%20Structure%20%28by%20ref%29))
  (if (Utilities|Enum|Equal(Enum) (Utilities|String|ToString(Name) (Utilities|Array|Get(acopy) (Variables|/Script/Engine.Actor|GetTags Other))) "Floor")
    (Utilities|FlowControl|DoOnce false
      (:Completed
        (bind _output_get (Variables|Default|SetHitPosition HitLocation))
        (Development|SetHiddeninGame (Variables|Default|GetParticleSystem) true false)
        (bind _returnvalue (Effects|SpawnEmitteratLocation "/Game/ClashRoyaleTest/Effect/P_fazhen_fire.P_fazhen_fire" (Math|Vector|MakeVector (.X (Math|Vector|BreakVector _output_get)) (.Y (Math|Vector|BreakVector _output_get)) (+ (.Z (Math|Vector|BreakVector _output_get)) 1.0))))
        (Transformation|SetWorldScale3D _returnvalue "4.000000,4.000000,4.000000")
        (Utilities|FlowControl|Delay 1.0)
        (Components|DestroyComponent _returnvalue)
        (bind _returnvalue_2 (Effects|SpawnEmitteratLocation "/Game/ClashRoyaleTest/Effect/P_yunshishu.P_yunshishu" _output_get (Variables|Default|GetSkillRotaion)))
        (Transformation|SetWorldScale3D _returnvalue_2 "2.000000,2.000000,2.000000")
        ;[1 1 1] Meteorite Damage is Complex
        (Utilities|FlowControl|Delay 1.2)
        (Variables|Default|SetStartFireImpulse true)
        (Game|Damage|ApplyRadialDamage 275.0 _output_get 1e+02 (Utilities|Select :Index (Variables|Default|GetCamp) :NewEnumerator0 "/Game/ClashRoyaleTest/Blueprints/CommonDefine/BP_CampDamageType_Blue.BP_CampDamageType_Blue_C" :NewEnumerator1 "/Game/ClashRoyaleTest/Blueprints/CommonDefine/BP_CampDamageType_Red.BP_CampDamageType_Red_C") 0 (Game|GetInstigator) 0 true "ECC_WorldDynamic")
        (Class|RadialForceComponent|FireImpulse (Variables|Default|GetRadialForce))
        (if (Variables|Default|GetIsDebug)
          (Rendering|Debug|DrawDebugCircle (Variables|Default|GetHitPosition) 1e+02 12 "(R=1.000000,G=0.121217,B=0.071455,A=1.000000)" 5.0 1.0 "0.000000,1.000000,0.000000" "1.000000,0.000000,0.000000" true))
        (Utilities|FlowControl|Delay 0.6)
        (Game|Damage|ApplyRadialDamage 81.0 (+ (Variables|Default|GetHitPosition) (* (Math|Vector|Normalize (Math|Vector|GetForwardVector (Variables|Default|GetSkillRotaion))) 1.2e+02)) 1e+02 (Utilities|Select :Index (Variables|Default|GetCamp) :NewEnumerator0 "/Game/ClashRoyaleTest/Blueprints/CommonDefine/BP_CampDamageType_Blue.BP_CampDamageType_Blue_C" :NewEnumerator1 "/Game/ClashRoyaleTest/Blueprints/CommonDefine/BP_CampDamageType_Red.BP_CampDamageType_Red_C") 0 (Game|GetInstigator) 0 true "ECC_WorldDynamic")
        (if (Variables|Default|GetIsDebug)
          (Rendering|Debug|DrawDebugCircle (+ (Variables|Default|GetHitPosition) (* (Math|Vector|Normalize (Math|Vector|GetForwardVector (Variables|Default|GetSkillRotaion))) 1.2e+02)) 1e+02 12 "(R=1.000000,G=0.121217,B=0.071455,A=1.000000)" 5.0 1.0 "0.000000,1.000000,0.000000" "1.000000,0.000000,0.000000" true))
        (Utilities|FlowControl|Delay 0.6)
        (Game|Damage|ApplyRadialDamage 81.0 (+ (Variables|Default|GetHitPosition) (* (Math|Vector|Normalize (Math|Vector|GetForwardVector (Variables|Default|GetSkillRotaion))) 2.4e+02)) 1e+02 (Utilities|Select :Index (Variables|Default|GetCamp) :NewEnumerator0 "/Game/ClashRoyaleTest/Blueprints/CommonDefine/BP_CampDamageType_Blue.BP_CampDamageType_Blue_C" :NewEnumerator1 "/Game/ClashRoyaleTest/Blueprints/CommonDefine/BP_CampDamageType_Red.BP_CampDamageType_Red_C") 0 (Game|GetInstigator) 0 true "ECC_WorldDynamic")
        (if (Variables|Default|GetIsDebug)
          (Rendering|Debug|DrawDebugCircle (+ (Variables|Default|GetHitPosition) (* (Math|Vector|Normalize (Math|Vector|GetForwardVector (Variables|Default|GetSkillRotaion))) 2.4e+02)) 1e+02 12 "(R=1.000000,G=0.121217,B=0.071455,A=1.000000)" 5.0 1.0 "0.000000,1.000000,0.000000" "1.000000,0.000000,0.000000" true))
        (Utilities|FlowControl|Delay 0.6)
        (Game|Damage|ApplyRadialDamage 81.0 (+ (Variables|Default|GetHitPosition) (* (Math|Vector|Normalize (Math|Vector|GetForwardVector (Variables|Default|GetSkillRotaion))) 3.6e+02)) 1e+02 (Utilities|Select :Index (Variables|Default|GetCamp) :NewEnumerator0 "/Game/ClashRoyaleTest/Blueprints/CommonDefine/BP_CampDamageType_Blue.BP_CampDamageType_Blue_C" :NewEnumerator1 "/Game/ClashRoyaleTest/Blueprints/CommonDefine/BP_CampDamageType_Red.BP_CampDamageType_Red_C") 0 (Game|GetInstigator) 0 true "ECC_WorldDynamic")
        (if (Variables|Default|GetIsDebug)
          (Rendering|Debug|DrawDebugCircle (+ (Variables|Default|GetHitPosition) (* (Math|Vector|Normalize (Math|Vector|GetForwardVector (Variables|Default|GetSkillRotaion))) 3.6e+02)) 1e+02 12 "(R=1.000000,G=0.121217,B=0.071455,A=1.000000)" 5.0 1.0 "0.000000,1.000000,0.000000" "1.000000,0.000000,0.000000" true))
        (Actor|DestroyActor)))))

(event EventTick
  (params (DeltaSeconds :type Float%20%28single-precision%29))
  (if (Variables|Default|GetStartFireImpulse)
    (Transformation|AddRelativeLocation (Variables|Default|GetRadialForce1) (Math|Vector|MakeVector (* DeltaSeconds 2.6e+02) 0.0 0.0) false false)
    (Class|RadialForceComponent|FireImpulse (Variables|Default|GetRadialForce1))))

(event EventSetSkillBallRotation
  (params (Rotation :type Rotator))
  (bind _output_get (Variables|Default|SetSkillRotaion Rotation))
  (Transformation|SetActorRotation _output_get))

(fn ConstructionScript
  (|CallParentFunction))