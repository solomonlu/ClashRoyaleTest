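; Soldiers skill ball that splits into a ring of smaller balls once it drops below a set height, then destroys itself.
; The construction script precomputes evenly spaced horizontal directions from the split count, despite the array's "Random" name.
; Tick watches the height and spawns one BP_SkillBall_Soldiers_Split per direction, each inheriting the sphere's physics velocity plus an outward push.
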(event EventTick
  (params (DeltaSeconds :type Float%20%28single-precision%29))
  (bind _returnvalue (Transformation|GetActorTransform))
  (if (< (.z (Transformation|GetActorLocation)) (Variables|Default|GetSplitZHeight))
    (Utilities|FlowControl|DoOnce false
      (:Completed
        (bind _returnvalue_2 (Physics|GetPhysicsLinearVelocity (Variables|Default|GetSphere) "None"))
        (while (> (Variables|Default|GetCurSplitBallCount_0) 0)
          (Math|Integer|DecrementInt (Variables|Default|GetCurSplitBallCount_0)
            (:%20%20
              (Game|SpawnActorfromClass "/Game/ClashRoyaleTest/Blueprints/SkillBall/Soldiers/BP_SkillBall_Soldiers_Split.BP_SkillBall_Soldiers_Split_C" (Math|Transform|MakeTransform (.location _returnvalue) (.rotation _returnvalue) (.scale _returnvalue)) "AlwaysSpawn" 0 (+ _returnvalue_2 (* (Utilities|Array|Get(acopy) (Variables|Default|GetRandomSplitBallVector_0) (Variables|Default|GetCurSplitBallCount_0)) 100)) 0))))
        (Actor|DestroyActor)))))

(fn ConstructionScript
  (|CallParentFunction)
  (bind _output_get (Variables|Default|SetCurSplitBallCount_0 (Variables|Default|GetSplitCount)))
  (LocalVariables|SetSplitAngular (Math|Conversions|ToFloat(Integer) (/ 360 (Variables|Default|GetSplitCount))))
  (while (> _output_get 0)
    (bind _result (Math|Integer|DecrementInt (Variables|Default|GetCurSplitBallCount_0))
      (:%20%20
        (Utilities|Array|Add (Variables|Default|GetRandomSplitBallVector_0) (Math|Vector|MakeVector (Math|Trig|Cos(Degrees) (* _result (LocalVariables|GetSplitAngular))) (Math|Trig|Sin(Degrees) (* _result (LocalVariables|GetSplitAngular))) 0.0)))))
  (Variables|Default|SetCurSplitBallCount_0 (Variables|Default|GetSplitCount)))