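; BP_SkillBall_SkeletonArcher is a skill ball that deploys skeleton archers for its Camp.
; When it falls below SplitZHeight, it spawns SplitCount split balls, each inheriting its velocity plus a scaled RandomSplitBallVector offset, then destroys itself.
; If it hits a Floor-tagged actor first, it instead spawns one archer, raised by half height and using the stored skill rotation, then destroys itself.
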(event Collision|EventHit
  (params (MyComp :type Primitive%20Component%20Object%20Reference) (Other :type Actor%20Object%20Reference) (OtherComp :type Primitive%20Component%20Object%20Reference) (bSelfMoved :type Boolean) (HitLocation :type Vector) (HitNormal :type Vector :default "0, 0, 0") (NormalImpulse :type Vector :default "0, 0, 0") (Hit :type Hit%20Result%20Structure%20%28by%20ref%29))
  (bind (_x _y _z) (Math|Vector|BreakVector HitLocation))
  (if (Utilities|Enum|Equal(Enum) (Utilities|String|ToString(Name) (Utilities|Array|Get(acopy) (Variables|/Script/Engine.Actor|GetTags Other))) "Floor")
    (Utilities|FlowControl|DoOnce false
      (:Completed
        (Game|SpawnActorfromClass "/Game/ClashRoyaleTest/Blueprints/SpawnObject/Soldiers/SkeletonArcher/BP_SkeletonArcher.BP_SkeletonArcher_C" (Math|Transform|MakeTransform (Math|Vector|MakeVector _x _y (+ _z 6e+01)) (Variables|Default|GetSkillRotaion) "1.000000,1.000000,1.000000") "Undefined" 0 (Variables|Default|GetCamp) 0)
        (Actor|DestroyActor)))))

(event EventTick
  (params (DeltaSeconds :type Float%20%28single-precision%29))
  (bind _returnvalue (Transformation|GetActorTransform))
  (|CallParentFunction DeltaSeconds)
  (if (< (.z (Transformation|GetActorLocation)) (Variables|Default|GetSplitZHeight))
    (Utilities|FlowControl|DoOnce false
      (:Completed
        (bind _returnvalue_2 (Physics|GetPhysicsLinearVelocity (Variables|Default|GetSphere) "None"))
        (while (> (Variables|Default|GetSplitCount) 0)
          (Math|Integer|DecrementInt (Variables|Default|GetSplitCount)
            (:%20%20
              (Game|SpawnActorfromClass "/Game/ClashRoyaleTest/Blueprints/SkillBall/Soldiers/BP_SkillBall_SkeletonArcher_Split.BP_SkillBall_SkeletonArcher_Split_C" (Math|Transform|MakeTransform (.location _returnvalue) (.rotation _returnvalue) (.scale _returnvalue)) "AlwaysSpawn" 0 (+ _returnvalue_2 (* (Utilities|Array|Get(acopy) (Variables|Default|GetRandomSplitBallVector) (Variables|Default|GetSplitCount)) 150)) (Variables|Default|GetCamp)))))
        (Actor|DestroyActor)))))

(event EventSetSkillBallRotation
  (params (Rotation :type Rotator))
  (Variables|Default|SetSkillRotaion Rotation))

(fn ConstructionScript
  (|CallParentFunction))