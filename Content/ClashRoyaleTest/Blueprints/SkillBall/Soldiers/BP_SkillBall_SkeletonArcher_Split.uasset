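; BP_SkillBall_SkeletonArcher_Split is a skill ball projectile that turns into a skeleton archer when it lands.
; Its construction script runs the parent's, then applies InitVelocity to the projectile movement.
; On the first hit against an actor whose first tag is Floor, it spawns BP_SkeletonArcher slightly above the impact point, passes on its Camp and destroys itself.
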(event Collision|EventHit
  (params (MyComp :type Primitive%20Component%20Object%20Reference) (Other :type Actor%20Object%20Reference) (OtherComp :type Primitive%20Component%20Object%20Reference) (bSelfMoved :type Boolean) (HitLocation :type Vector) (HitNormal :type Vector :default "0, 0, 0") (NormalImpulse :type Vector :default "0, 0, 0") (Hit :type Hit%20Result%20Structure%20%28by%20ref%29))
  (bind (_x _y _z) (Math|Vector|BreakVector HitLocation))
  (if (Utilities|Enum|Equal(Enum) (Utilities|String|ToString(Name) (Utilities|Array|Get(acopy) (Variables|/Script/Engine.Actor|GetTags Other))) "Floor")
    (Utilities|FlowControl|DoOnce false
      (:Completed
        (Game|SpawnActorfromClass "/Game/ClashRoyaleTest/Blueprints/SpawnObject/Soldiers/SkeletonArcher/BP_SkeletonArcher.BP_SkeletonArcher_C" (Math|Transform|MakeTransform (Math|Vector|MakeVector _x _y (+ _z 6e+01)) "0, 0, 0" "1.000000,1.000000,1.000000") "AdjustIfPossibleButAlwaysSpawn" 0 (Variables|Default|GetCamp) 0)
        (Actor|DestroyActor)))))

(fn ConstructionScript
  (|CallParentFunction)
  (Variables|/Script/Engine.MovementComponent|SetVelocity (Variables|Default|GetProjectileMovement) (Variables|Default|GetInitVelocity)))