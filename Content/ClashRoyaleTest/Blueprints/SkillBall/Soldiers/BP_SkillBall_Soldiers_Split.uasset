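; BP_SkillBall_Soldiers_Split is a projectile skill ball that deploys soldiers where it lands.
; On construction it sets its projectile movement velocity from InitVelocity.
; When it hits an actor whose first tag is Floor, a DoOnce gate lets it spawn one BP_Soldiers actor at the hit location, then the ball destroys itself.
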(event Collision|EventHit
  (params (MyComp :type Primitive%20Component%20Object%20Reference) (Other :type Actor%20Object%20Reference) (OtherComp :type Primitive%20Component%20Object%20Reference) (bSelfMoved :type Boolean) (HitLocation :type Vector) (HitNormal :type Vector :default "0, 0, 0") (NormalImpulse :type Vector :default "0, 0, 0") (Hit :type Hit%20Result%20Structure%20%28by%20ref%29))
  (if (Utilities|Enum|Equal(Enum) (Utilities|String|ToString(Name) (Utilities|Array|Get(acopy) (Variables|/Script/Engine.Actor|GetTags Other))) "Floor")
    (Utilities|FlowControl|DoOnce false
      (:Completed
        (Game|SpawnActorfromClass "/Game/ClashRoyaleTest/Blueprints/SpawnObject/Soldiers/BP_Soldiers.BP_Soldiers_C" (Math|Transform|MakeTransform HitLocation "0, 0, 0" "1.000000,1.000000,1.000000") "Undefined" 0 0)
        (Actor|DestroyActor)))))

(fn ConstructionScript
  (|CallParentFunction)
  (Variables|/Script/Engine.MovementComponent|SetVelocity (Variables|Default|GetProjectileMovement) (Variables|Default|GetInitVelocity)))