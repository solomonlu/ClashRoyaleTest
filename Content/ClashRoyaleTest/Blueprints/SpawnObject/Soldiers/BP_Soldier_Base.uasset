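; Base soldier character for a Clash Royale-style game, with a Blue or Red camp, health, cooldown-gated attacks and death.
; Construction loads stats from DT_SoldierProperty; after an activation delay, BeginPlay enables the behavior tree through the Blackboard.
; Attack range selects melee damage or homing bullets, with camp-specific damage types filtering out friendly fire.
; Death disables AI and collision before timed removal, a player-facing indicator shows health, and colliding soldiers receive impulses.
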(event OnPerceptionUpdated(AIPerception)
  (params (UpdatedActors :type Array%20of%20Actor%20Object%20References))
  ;[1 1 1] can't see the building placed in the map.WHY!!!
)

(event OnComponentHit(CapsuleComponent)
  (params (HitComponent :type Primitive%20Component%20Object%20Reference) (OtherActor :type Actor%20Object%20Reference) (OtherComp :type Primitive%20Component%20Object%20Reference) (NormalImpulse :type Vector) (Hit :type Hit%20Result%20Structure%20%28by%20ref%29))
  ;[1 1 1] on collision with other soldiers
  (bind _asbp_soldier_base (Utilities|Casting|CastToBP_Soldier_Base OtherActor))
  (Physics|AddImpulse (Variables|/Script/Engine.Character|GetCharacterMovement _asbp_soldier_base) (* (.Normal (Collision|BreakHitResult Hit)) -2.5e+02) true))

(event Custom|Attack!
  ;[1 1 1] Attack!
  (bind _canattack (CallFunction|CanAttack))
  (if _canattack
    (if (> (Variables|Attack|GetAttackRange) 2e+02)
      (CallFunction|AttackinRange)
      (else
        (CallFunction|AttackinMelee)))
    (Variables|Attack|SetAttackCoolDown (Variables|Attack|GetAttackSpeed))))

(event Custom|OnDeath
  ;[1 1 1] damage deal
  (Variables|Common|SetIsDead true)
  (Variables|/Script/Engine.CharacterMovementComponent|SetMaxWalkSpeed (Variables|Character|GetCharacterMovement) 0.0)
  (Collision|SetCollisionEnabled (Variables|Collision|GetCapsuleComponent) "NoCollision")
  (AI|Components|Blackboard|SetValueasBool (AI|GetBlackboard 0) (Utilities|Name|MakeLiteralName "IsBehaviorTreeEnabled") false)
  (bind _asaicontroller (Utilities|Casting|CastToAIController (Pawn|GetController))
    (:then
      (AI|ClearFocus _asaicontroller))
    (:CastFailed
      _))
  (Actor|SetLifeSpan 2.0))

(event EventBeginPlay
  (Variables|Common|SetCurHealth (Math|Conversions|ToFloat(Integer) (Variables|Common|GetMaxHealth)))
  ;[1 1 1] Active Time.
  (Utilities|FlowControl|Delay (Variables|Common|GetActiveDelay))
  (AI|Components|Blackboard|SetValueasBool (AI|GetBlackboard 0) (Utilities|Name|MakeLiteralName "IsBehaviorTreeEnabled") true)
  (AI|Components|Blackboard|SetValueasFloat (AI|GetBlackboard 0) (Utilities|Name|MakeLiteralName "AttackRange") (Variables|Attack|GetAttackRange)))

(event Game|Damage|EventAnyDamage
  (params (Damage :type Float%20%28single-precision%29) (DamageType :type Damage%20Type%20Object%20Reference) (InstigatedBy :type Controller%20Object%20Reference) (DamageCauser :type Actor%20Object%20Reference))
  (bind (_asbp_camp_damage_type _bsuccess) (Utilities|Casting|CastToBP_CampDamageType DamageType))
  ;[1 1 1] damage deal
  (if (not (Variables|Common|GetIsDead))
    (if (and _bsuccess (Utilities|Enum|NotEqual(Enum) (Variables|/Game/ClashRoyaleTest/Blueprints/CommonDefine/BP_CampDamageType.BP_CampDamageType_C|GetCamp _asbp_camp_damage_type) (Variables|Common|GetCamp)))
      (bind _output_get (Variables|Common|SetCurHealth (Math|Float|Clamp(Float) (- (Variables|Common|GetCurHealth) Damage) 0.0 (Math|Conversions|ToFloat(Integer) (Variables|Common|GetMaxHealth)))))
      (if (<= _output_get 0.0)
        (CallFunction|OnDeath)))))

(event EventTick
  (params (DeltaSeconds :type Float%20%28single-precision%29))
  (Utilities|FlowControl|Sequence
    (:then_0
      ;[1 1 1] If have cooldown,then reduce it
      (if (> (Variables|Attack|GetAttackCoolDown) 0.0)
        (Variables|Attack|SetAttackCoolDown (- (Variables|Attack|GetAttackCoolDown) DeltaSeconds))))
    (:then_2
      ;[1 1 1] always face to the player
      (Transformation|SetWorldRotation (Variables|Default|GetHealthIndicator) (Math|Rotator|FindLookatRotation (Transformation|GetActorLocation) (Transformation|GetActorLocation (Game|Player|GetPlayerPawn 0))) false false))))

(fn ConstructionScript
  (Effects|Components|ParticleSystem|SetTemplate (Variables|Default|GetCampIndicator) (Utilities|Select :Index (Variables|Common|GetCamp) :NewEnumerator0 "/Game/ClashRoyaleTest/Effect/P_bluequan.P_bluequan" :NewEnumerator1 "/Game/ClashRoyaleTest/Effect/P_redquan.P_redquan"))
  ;[1 1 1] read property from table
  (bind _returnvalue (Utilities|GetDataTableRow "/Game/ClashRoyaleTest/Blueprints/GameDesign/DT_SoldierProperty.DT_SoldierProperty" (Utilities|String|StringToName (Variables|Common|GetSoldierName)))
    (:then
      (Utilities|FlowControl|Sequence
        (:then_0
          (Variables|Common|SetMaxHealth (.MaxHealth (Utilities|Struct|BreakS_SoldierPropertyDataTable _returnvalue))))
        (:then_1
          (bind _output_get (Variables|Common|SetMoveSpeed (.WalkSpeed (Utilities|Struct|BreakS_SoldierPropertyDataTable _returnvalue))))
          (Variables|/Script/Engine.CharacterMovementComponent|SetMaxWalkSpeed (Variables|Character|GetCharacterMovement) _output_get))
        (:then_2
          (Variables|Attack|SetAttackDamage (.AttackDamage (Utilities|Struct|BreakS_SoldierPropertyDataTable _returnvalue))))
        (:then_3
          (Variables|Attack|SetAttackSpeed (.AttackSpeed (Utilities|Struct|BreakS_SoldierPropertyDataTable _returnvalue))))
        (:then_4
          (Variables|Attack|SetAttackRange (.AttackRange (Utilities|Struct|BreakS_SoldierPropertyDataTable _returnvalue))))
        (:then_5
          (Variables|Attack|SetAttackMode (.AttackMode (Utilities|Struct|BreakS_SoldierPropertyDataTable _returnvalue))))
        (:then_6
          (Variables|Common|SetActiveDelay (.ActiveDelay (Utilities|Struct|BreakS_SoldierPropertyDataTable _returnvalue))))))))

(fn OnRepCurHealth
  (bind _curhealth (Variables|Common|GetCurHealth))
  (bind _maxhealth (Variables|Common|GetMaxHealth))
  (bind _returnvalue (Math|Conversions|ToFloat(Integer) _maxhealth))
  (Rendering|Material|SetScalarParameterValueonMaterials (Variables|Default|GetHealthIndicator) "Energy" (/ _curhealth _returnvalue))
  (Development|SetHiddeninGame (Variables|Default|GetHealthIndicator) (== _curhealth _returnvalue) false))

(fn CanAttack
  (return (<= (Variables|Attack|GetAttackCoolDown) 0.0)))

(fn AttackinMelee
  (bind _attacktarget (Variables|Attack|GetAttackTarget))
  (Variables|Attack|SetIsAttacking false)
  (Utilities|IsValid _attacktarget
    (:Is%20Valid
      (if (Utilities|DoesObjectImplementInterface _attacktarget "/Game/ClashRoyaleTest/Blueprints/SpawnObject/BPI_SoldiersAndBuildingsInterface.BPI_SoldiersAndBuildingsInterface_C")
        (bind _isdead (Class|BPISoldiersandBuildingsInterface|GetIsDead(Message) _attacktarget))
        (if (not _isdead)
          (Game|Damage|ApplyDamage (Variables|Attack|GetAttackTarget) (Variables|Attack|GetAttackDamage) 0 self (Utilities|Select :Index (Variables|Common|GetCamp) :NewEnumerator0 "/Game/ClashRoyaleTest/Blueprints/CommonDefine/BP_CampDamageType_Blue.BP_CampDamageType_Blue_C" :NewEnumerator1 "/Game/ClashRoyaleTest/Blueprints/CommonDefine/BP_CampDamageType_Red.BP_CampDamageType_Red_C")))))))

(fn AttackinRange
  (bind _attacktarget (Variables|Attack|GetAttackTarget))
  (Variables|Attack|SetIsAttacking false)
  (Utilities|IsValid _attacktarget
    (:Is%20Valid
      (if (Utilities|DoesObjectImplementInterface _attacktarget "/Game/ClashRoyaleTest/Blueprints/SpawnObject/BPI_SoldiersAndBuildingsInterface.BPI_SoldiersAndBuildingsInterface_C")
        (bind _isdead (Class|BPISoldiersandBuildingsInterface|GetIsDead(Message) _attacktarget))
        (if (not _isdead)
          (bind _returnvalue (Game|SpawnActorfromClass (Variables|Attack|GetRangeAttackBullet) (Math|Transform|MakeTransform (Transformation|GetSocketLocation (Variables|Character|GetMesh self) "EmitSocket") (Transformation|GetActorRotation) "2.000000,2.000000,2.000000") "Undefined" 0 self))
          (if (Utilities|DoesObjectImplementInterface _returnvalue "/Game/ClashRoyaleTest/Blueprints/SpawnObject/Bullet/BPI_BulletInterface.BPI_BulletInterface_C")
            (Class|BPIBulletInterface|SetDamage(Message) _returnvalue (Variables|Attack|GetAttackDamage))
            (Class|BPIBulletInterface|SetHomingTarget(Message) _returnvalue (Variables|Attack|GetAttackTarget))
            (Class|BPIBulletInterface|SetCamp(Message) _returnvalue (Variables|Common|GetCamp))))))))

(fn SetinAttacking
  (Variables|Attack|SetIsAttacking true))

(fn DistancetoTarget
  (bind _outhit (Collision|LineTraceByChannel (Transformation|GetActorLocation) (Transformation|GetActorLocation (Variables|Attack|GetAttackTarget)) "TraceTypeQuery1" false (Utilities|Array|MakeArray self) "None"))
  (if (== (.HitActor (Collision|BreakHitResult _outhit)) (Variables|Attack|GetAttackTarget))
    (return (Math|Vector|VectorLength (- (.ImpactPoint (Collision|BreakHitResult _outhit)) (Transformation|GetActorLocation))))
    (else
      (return (Math|Vector|VectorLength (- (Transformation|GetActorLocation (Variables|Attack|GetAttackTarget)) (Transformation|GetActorLocation)))))))

(fn GetCamp
  (return (Variables|Common|GetCamp)))

(fn GetIsDead
  (return (Variables|Common|GetIsDead)))