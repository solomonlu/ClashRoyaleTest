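; Centaur soldier that charges at distant attack targets and shoves aside other soldiers it bumps into.
; While the target is out of range, Tick runs down a cooldown, then RushSwitch doubles walk speed and sets the IsRushing blackboard key.
; Paired DoOnce gates end the rush on reaching range and restart the cooldown.
; Collision impulses are stronger while rushing, and a helper deals double damage with a camp-specific damage type.
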(event OnComponentHit(CapsuleComponent)
  (params (HitComponent :type Primitive%20Component%20Object%20Reference) (OtherActor :type Actor%20Object%20Reference) (OtherComp :type Primitive%20Component%20Object%20Reference) (NormalImpulse :type Vector :default "0, 0, 0") (Hit :type Hit%20Result%20Structure%20%28by%20ref%29))
  (bind _normal (Collision|BreakHitResult Hit))
  (bind _asbp_soldier_base (Utilities|Casting|CastToBP_Soldier_Base OtherActor))
  (if (not (== _asbp_soldier_base (Variables|Default|GetAttackTarget)))
    (if (Variables|Default|GetIsRushing)
      (Physics|AddImpulse (Variables|/Script/Engine.Character|GetCharacterMovement _asbp_soldier_base) (* _normal -4e+02) true)
      (else
        (Physics|AddImpulse (Variables|/Script/Engine.Character|GetCharacterMovement _asbp_soldier_base) (* _normal -2.5e+02) true)))))

(event EventTick
  (params (DeltaSeconds :type Float%20%28single-precision%29))
  (|CallParentFunction DeltaSeconds)
  (Utilities|IsValid (Variables|Default|GetAttackTarget)
    (:Is%20Valid
      (bind _distance (CallFunction|DistancetoTarget))
      (if (> _distance (Variables|Default|GetAttackRange))
        (bind _output_get (Variables|Default|SetRushSwitchCooldown (Math|Float|Clamp(Float) (- (Variables|Default|GetRushSwitchCooldown) DeltaSeconds) 0.0 (Variables|Default|GetRushSwitchTime))))
        (if (== _output_get 0.0)
          (Utilities|FlowControl|DoOnce false :!label _label
            (:Completed
              (Utilities|FlowControl|Delay 0.2)
              (CallFunction|RushSwitch true)
              (goto _label_2 Reset))))
        (else
          (Utilities|FlowControl|DoOnce false :!label _label_2
            (:Completed
              (Variables|Default|SetRushSwitchCooldown (Variables|Default|GetRushSwitchTime))
              (Utilities|FlowControl|Delay 0.2)
              (CallFunction|RushSwitch false)
              (goto _label Reset))))))))

(fn ConstructionScript
  (|CallParentFunction))

(fn RushSwitch
  (params (To :type Boolean))
  (bind _output_get (Variables|Default|SetIsRushing To))
  (AI|Components|Blackboard|SetValueasBool (AI|GetBlackboard 0) (Utilities|Name|MakeLiteralName "IsRushing") _output_get)
  (if _output_get
    (Variables|/Script/Engine.CharacterMovementComponent|SetMaxWalkSpeed (Variables|Character|GetCharacterMovement) (* 2 (Variables|Default|GetMoveSpeed)))
    (else
      (Variables|/Script/Engine.CharacterMovementComponent|SetMaxWalkSpeed (Variables|Character|GetCharacterMovement) (Variables|Default|GetMoveSpeed)))))

(fn CauseDoubleDamagetoTarget
  (Game|Damage|ApplyDamage (Variables|Default|GetAttackTarget) (* 2 (Variables|Default|GetAttackDamage)) 0 self (Utilities|Select :Index (Variables|Default|GetCamp) :NewEnumerator0 "/Game/ClashRoyaleTest/Blueprints/CommonDefine/BP_CampDamageType_Blue.BP_CampDamageType_Blue_C" :NewEnumerator1 "/Game/ClashRoyaleTest/Blueprints/CommonDefine/BP_CampDamageType_Red.BP_CampDamageType_Red_C")))