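; BP_FemaleMage is a Female Mage soldier Blueprint whose construction script only calls its parent.
; ShootTarget is an empty override, so this graph fires nothing.
; Disconnected logic marked UNUSE would spawn a homing frost bolt at EmitSocket for a living target, passing damage, target and camp through BPI_BulletInterface and deriving lifespan from attack range and projectile speed.
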(fn ConstructionScript
  (|CallParentFunction))

(fn ShootTarget)