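; Archer bow projectile that damages one assigned target, with damage amount, target and camp set through events.
; On begin or end overlap with that target, it applies damage with a blue or red camp damage type, then destroys itself.
; The construction script makes the mesh ignore its owner when moving.
; Homing setup toward soldier capsules or building boxes exists in the graph but is disconnected and never runs.
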(event OnComponentBeginOverlap(StaticMesh)
  (params (OverlappedComponent :type Primitive%20Component%20Object%20Reference) (OtherActor :type Actor%20Object%20Reference) (OtherComp :type Primitive%20Component%20Object%20Reference) (OtherBodyIndex :type Integer) (bFromSweep :type Boolean) (SweepResult :type Hit%20Result%20Structure%20%28by%20ref%29))
  (if (== OtherActor (Variables|Default|GetHomingTarget))
    (Game|Damage|ApplyDamage OtherActor (Variables|Default|GetDamage) 0 (Game|GetInstigator) (Utilities|Select :Index (Variables|Default|GetCamp) :NewEnumerator0 "/Game/ClashRoyaleTest/Blueprints/CommonDefine/BP_CampDamageType_Blue.BP_CampDamageType_Blue_C" :NewEnumerator1 "/Game/ClashRoyaleTest/Blueprints/CommonDefine/BP_CampDamageType_Red.BP_CampDamageType_Red_C"))
    (Actor|DestroyActor) ; Then destroy this projectile
  ))

(event OnComponentEndOverlap(StaticMesh)
  (params (OverlappedComponent :type Primitive%20Component%20Object%20Reference) (OtherActor :type Actor%20Object%20Reference) (OtherComp :type Primitive%20Component%20Object%20Reference) (OtherBodyIndex :type Integer))
  (if (== OtherActor (Variables|Default|GetHomingTarget))
    (Game|Damage|ApplyDamage OtherActor (Variables|Default|GetDamage) 0 (Game|GetInstigator) (Utilities|Select :Index (Variables|Default|GetCamp) :NewEnumerator0 "/Game/ClashRoyaleTest/Blueprints/CommonDefine/BP_CampDamageType_Blue.BP_CampDamageType_Blue_C" :NewEnumerator1 "/Game/ClashRoyaleTest/Blueprints/CommonDefine/BP_CampDamageType_Red.BP_CampDamageType_Red_C"))
    (Actor|DestroyActor) ; Then destroy this projectile
  ))

(event EventSetDamage
  (params (Damage :type Float%20%28single-precision%29))
  (Variables|Default|SetDamage Damage))

(event EventSetHomingTarget
  (params (Target :type Actor%20Object%20Reference))
  (Variables|Default|SetHomingTarget Target))

(event EventSetCamp
  (params (Camp :type E_Camp%20Enum :default "NewEnumerator0"))
  (Variables|Default|SetCamp Camp))

(fn ConstructionScript
  (Collision|IgnoreActorwhenMoving (Variables|Default|GetStaticMesh) (Components|GetOwner) true))