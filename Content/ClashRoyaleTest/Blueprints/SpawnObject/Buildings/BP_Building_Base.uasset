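; Base building actor for a Clash Royale-style game that belongs to a camp and takes damage only from other camps' BP_CampDamageType.
; Tick runs three cooldowns: periodic health bleed, optional attacks and optional soldier spawning at set positions.
; Attacks fire homing bullets configured through an interface, reacquiring the nearest in-range enemy by sphere overlap when the target is invalid.
; CurHealth's RepNotify drives the health indicator; zero health destroys the actor.
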(event Custom|OnDeath
  ;[1 1 1] damage deal
  (CallFunction|HandleonDead))

(event Game|Damage|EventAnyDamage
  (params (Damage :type Float%20%28single-precision%29) (DamageType :type Damage%20Type%20Object%20Reference) (InstigatedBy :type Controller%20Object%20Reference) (DamageCauser :type Actor%20Object%20Reference))
  (bind (_asbp_camp_damage_type _bsuccess) (Utilities|Casting|CastToBP_CampDamageType DamageType))
  ;[1 1 1] damage deal
  (if (not (Variables|Common|GetIsDead))
    (if (and _bsuccess (Utilities|Enum|NotEqual(Enum) (Variables|/Game/ClashRoyaleTest/Blueprints/CommonDefine/BP_CampDamageType.BP_CampDamageType_C|GetCamp _asbp_camp_damage_type) (Variables|Common|GetCamp)))
      (bind _output_get (Variables|Common|SetCurHealth (Math|Float|Clamp(Float) (- (Variables|Common|GetCurHealth) Damage) 0.0 (Math|Conversions|ToFloat(Integer) (Variables|Common|GetMaxHealth)))))
      (if (<= _output_get 0.0)
        (CallFunction|OnDeath)))))

(event EventTick
  (params (DeltaSeconds :type Float%20%28single-precision%29))
  (Utilities|FlowControl|Sequence
    (:then_0
      (if (<= (Variables|Common|GetBleedingCooldown) 0.0)
        (CallFunction|DoBleeding)
        (Variables|Common|SetBleedingCooldown (Variables|Common|GetBleedingInterval))
        (else
          ;[1 1 1] If have cooldown,then reduce it
          (Variables|Common|SetBleedingCooldown (- (Variables|Common|GetBleedingCooldown) DeltaSeconds)))))
    (:then_1
      (if (Variables|Attack|GetIsAttackBuilding)
        (if (<= (Variables|Attack|GetAttackCooldown) 0.0)
          (Utilities|IsValid (Variables|Attack|GetAttackTarget)
            (:Is%20Valid
              (if (<= (Transformation|GetDistanceTo (Variables|Attack|GetAttackTarget) self) (Variables|Attack|GetAttackRange))
                (if (Utilities|DoesObjectImplementInterface (Variables|Attack|GetAttackTarget) "/Game/ClashRoyaleTest/Blueprints/SpawnObject/BPI_SoldiersAndBuildingsInterface.BPI_SoldiersAndBuildingsInterface_C")
                  (bind _isdead (Class|BPISoldiersandBuildingsInterface|GetIsDead(Message) (Variables|Attack|GetAttackTarget)))
                  (if (not _isdead)
                    (CallFunction|AttacktoTarget)
                    (Variables|Attack|SetAttackCooldown (Variables|Attack|GetAttackSpeed))
                    (else
                      ;[1 1 1] if no target or target move out of range or dead,find new targe
                      (Variables|Attack|SetAttackTarget 0 :!label _label)
                      (CallFunction|FindClosestEnemy)))
                  (else
                    (goto _label)))
                (else
                  (goto _label))))
            (:Is%20Not%20Valid
              (goto _label)))
          (else
            ;[1 1 1] If have cooldown,then reduce it
            (Variables|Attack|SetAttackCooldown (- (Variables|Attack|GetAttackCooldown) DeltaSeconds))))))
    (:then_2
      (if (Variables|Spawn|GetIsSpawnBuilding)
        (if (<= (Variables|Spawn|GetSpawnCooldown) 0.0)
          (CallFunction|SpawnSoldier)
          (Variables|Spawn|SetSpawnCooldown (Variables|Spawn|GetSpawnInterval))
          (else
            ;[1 1 1] If have cooldown,then reduce it
            (Variables|Spawn|SetSpawnCooldown (- (Variables|Spawn|GetSpawnCooldown) DeltaSeconds))))))))

(event EventBeginPlay
  (Variables|Common|SetCurHealth (Math|Conversions|ToFloat(Integer) (Variables|Common|GetMaxHealth)))
  (Transformation|SetWorldRotation (Variables|Default|GetHealthIndicator) (Math|Rotator|FindLookatRotation (Transformation|GetActorLocation) (Transformation|GetActorLocation (Game|Player|GetPlayerPawn 0))) false false))

(fn ConstructionScript)

(fn OnRepCurHealth
  (bind _curhealth (Variables|Common|GetCurHealth))
  (bind _maxhealth (Variables|Common|GetMaxHealth))
  (bind _returnvalue (Math|Conversions|ToFloat(Integer) _maxhealth))
  (Rendering|Material|SetScalarParameterValueonMaterials (Variables|Default|GetHealthIndicator) "Energy" (/ _curhealth _returnvalue))
  (Development|SetHiddeninGame (Variables|Default|GetHealthIndicator) (== _curhealth _returnvalue) false))

(fn HandleonDead
  (Variables|Common|SetIsDead true)
  (Actor|DestroyActor))

(fn AttacktoTarget
  (bind _returnvalue (Transformation|GetActorTransform))
  (bind _bulletemitposition (Variables|Attack|GetBulletEmitPosition))
  (bind _returnvalue_2 (Math|Transform|TransformLocation _returnvalue _bulletemitposition))
  (bind _returnvalue_3 (Game|SpawnActorfromClass (Variables|Attack|GetAttackBulletClass) (Math|Transform|MakeTransform _returnvalue_2 (Math|Rotator|FindLookatRotation _returnvalue_2 (Transformation|GetActorLocation (Variables|Attack|GetAttackTarget))) "1,1,1") "Undefined" self 0))
  (if (Utilities|DoesObjectImplementInterface _returnvalue_3 "/Game/ClashRoyaleTest/Blueprints/SpawnObject/Bullet/BPI_BulletInterface.BPI_BulletInterface_C")
    (Class|BPIBulletInterface|SetDamage(Message) _returnvalue_3 (Variables|Attack|GetAttackDamage))
    (Class|BPIBulletInterface|SetHomingTarget(Message) _returnvalue_3 (Variables|Attack|GetAttackTarget))
    (Class|BPIBulletInterface|SetCamp(Message) _returnvalue_3 (Variables|Common|GetCamp))))

(fn FindClosestEnemy
  (LocalVariables|SetTempTargetDistance (Variables|Attack|GetAttackRange))
  (bind (_outactors _returnvalue) (Class|KismetSystemLibrary|SphereOverlapActorsNEW (Transformation|GetActorLocation) (Variables|Attack|GetAttackRange) (Utilities|Array|MakeArray "ObjectTypeQuery3") 0 (Utilities|Array|MakeArray self)))
  (if _returnvalue
    (for _array_element _outactors
      (if (Utilities|DoesObjectImplementInterface _array_element "/Game/ClashRoyaleTest/Blueprints/SpawnObject/BPI_SoldiersAndBuildingsInterface.BPI_SoldiersAndBuildingsInterface_C")
        (bind _camp (Class|BPISoldiersandBuildingsInterface|GetCamp(Message) _array_element))
        (if (Utilities|Enum|NotEqual(Enum) _camp (Variables|Common|GetCamp))
          (if (< (Transformation|GetDistanceTo _array_element self) (LocalVariables|GetTempTargetDistance))
            (LocalVariables|SetIsFindTarge true)
            (LocalVariables|SetTempTargetDistance (Transformation|GetDistanceTo _array_element self))
            (LocalVariables|SetTempTarget _array_element)))))
    (if (LocalVariables|GetIsFindTarge)
      (Variables|Attack|SetAttackTarget (LocalVariables|GetTempTarget))
      (return)
      (else
        (return)))
    (else
      (return))))

(fn SpawnSoldier
  (for _array_element (Variables|Spawn|GetSpawnPosition)
    (Game|SpawnActorfromClass (Variables|Spawn|GetSpawnSoldierClass) (Math|Transform|MakeTransform (Math|Transform|TransformLocation (Transformation|GetActorTransform) _array_element) (Math|Rotator|FindLookatRotation (Transformation|GetActorLocation) (Math|Transform|TransformLocation (Transformation|GetActorTransform) _array_element)) "1,1,1") "Undefined" 0 (Variables|Common|GetCamp) 0)))

(fn DoBleeding
  ;[1 1 1] common bleeding
  (bind _output_get (Variables|Common|SetCurHealth (Math|Float|Clamp(Float) (- (Variables|Common|GetCurHealth) (Variables|Common|GetBleedingHealthCount)) 0.0 (Math|Conversions|ToFloat(Integer) (Variables|Common|GetMaxHealth)))))
  (if (== _output_get 0.0)
    (Utilities|FlowControl|DoOnce false
      (:Completed
        (CallFunction|OnDeath))))
  (return))

(fn GetCamp
  (return (Variables|Common|GetCamp)))

(fn GetIsDead
  (return (Variables|Common|GetIsDead)))