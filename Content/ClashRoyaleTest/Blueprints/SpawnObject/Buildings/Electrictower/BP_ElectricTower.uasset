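; BP_ElectricTower is an electric tower building in the ClashRoyaleTest project that acquires enemy soldiers as attack targets.
; When a BP_Soldier_Base of a different Camp begins overlapping its Sphere, that actor becomes AttackTarget, replacing any previous one without a check.
; Death handling, Tick and construction only call the parent, and no attack logic appears in this Blueprint.
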(event OnComponentBeginOverlap(Sphere)
  (params (OverlappedComponent :type Primitive%20Component%20Object%20Reference) (OtherActor :type Actor%20Object%20Reference) (OtherComp :type Primitive%20Component%20Object%20Reference) (OtherBodyIndex :type Integer) (bFromSweep :type Boolean) (SweepResult :type Hit%20Result%20Structure%20%28by%20ref%29))
  (bind _asbp_soldier_base (Utilities|Casting|CastToBP_Soldier_Base OtherActor))
  (if (Utilities|Enum|NotEqual(Enum) (Variables|/Game/ClashRoyaleTest/Blueprints/SpawnObject/Soldiers/BP_Soldier_Base.BP_Soldier_Base_C|GetCamp _asbp_soldier_base) (Variables|Default|GetCamp))
    (Variables|Default|SetAttackTarget OtherActor)))

(event EventHandleonDead
  (|CallParentFunction))

(event EventTick
  (params (DeltaSeconds :type Float%20%28single-precision%29))
  (|CallParentFunction DeltaSeconds))

(fn ConstructionScript
  (|CallParentFunction))