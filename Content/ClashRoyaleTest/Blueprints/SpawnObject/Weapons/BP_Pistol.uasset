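; BP_Pistol is an interactable pistol weapon that spawns a BP_PistolBullet at its Arrow component's transform when used.
; Pickup disables gravity and sets very high damping on the mesh, while drop restores both and applies linear and angular impulses as velocity changes.
; It requests snapping to the interactor with a fixed attach offset and rotation, and both CanPickup and CanDrop return false.
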(event EventOnPickup
  (params (Interactor :type World%20Interactor%20Object%20Reference))
  (bind _pistolmesh (Variables|Default|GetPistolMesh))
  (Physics|SetEnableGravity _pistolmesh false)
  (Variables|Default|SetPreviousLinearDamping (Class|PrimitiveComponent|GetLinearDamping _pistolmesh))
  (Variables|Default|SetPreviousAngularDamping (Class|PrimitiveComponent|GetAngularDamping _pistolmesh))
  (Class|PrimitiveComponent|SetLinearDamping _pistolmesh 9999999999.0)
  (Class|PrimitiveComponent|SetAngularDamping _pistolmesh 99999999.0))

(event EventOnDrop
  (params (Velocity :type Vector) (AngularVelocity :type Vector) (Interactor :type World%20Interactor%20Object%20Reference))
  (bind _pistolmesh (Variables|Default|GetPistolMesh))
  (Class|PrimitiveComponent|SetLinearDamping _pistolmesh (Variables|Default|GetPreviousLinearDamping))
  (Class|PrimitiveComponent|SetAngularDamping _pistolmesh (Variables|Default|GetPreviousAngularDamping))
  (Physics|SetEnableGravity _pistolmesh true)
  (Physics|AddImpulse _pistolmesh Velocity "None" true)
  (Class|PrimitiveComponent|AddAngularImpulse _pistolmesh AngularVelocity "None" true))

(event EventOnUse
  (bind _arrow (Variables|Default|GetArrow))
  (Game|SpawnActorfromClass "/Game/ClashRoyaleTest/Blueprints/SpawnObject/Bullet/WeaponBullet/BP_PistolBullet.BP_PistolBullet_C" (Math|Transform|MakeTransform (Transformation|GetWorldLocation _arrow) (Transformation|GetWorldRotation _arrow) "1,1,1") "Undefined" 0 0))

(fn ConstructionScript)

(fn CanDrop
  (return false))

(fn CanPickup
  (return false))

(fn GetAttachLocation
  (return "10.353254, 0,0.914016"))

(fn GetAttachRotation
  (return "55.000000, 0, 0"))

(fn ShouldSnaptoInteractor
  (return true))