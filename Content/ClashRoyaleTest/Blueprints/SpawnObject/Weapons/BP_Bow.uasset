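; Bow weapon that an interactor holds and draws by dragging the string to spawn and fire BP_Bow_Bullet arrows, singly or as a multi-shot spread.
; Dragging from an "Emitter"-tagged sphere stretches two scaled string meshes, spawns arrows past a draw threshold and keeps them aimed.
; Release launches them at a speed proportional to draw distance, then a timeline snaps the string back and re-arms spawning.
; Pickup freezes physics with extreme damping.
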(event Custom|UpdateString
  (params (CenterPosition :type Vector))
  (bind _returnvalue (* 1.0 0.003))
  (bind _end2 (Variables|Default|Getend2))
  (bind _end1 (Variables|Default|Getend1))
  (bind _returnvalue_2 (Transformation|GetWorldLocation _end2))
  (bind _returnvalue_3 (Transformation|GetWorldLocation _end1))
  (Utilities|FlowControl|Sequence
    (:then_0
      ;[1 1 1] update the string
      (Transformation|SetWorldTransform (Variables|Default|Getstring2) (Math|Transform|MakeTransform (* (+ CenterPosition _returnvalue_2) 0.5) (Math|Rotator|FindLookatRotation CenterPosition _returnvalue_2) (Math|Vector|MakeVector (* (Math|Vector|VectorLength (- CenterPosition _returnvalue_2)) 0.01) _returnvalue _returnvalue)) false false)
      (Transformation|SetWorldTransform (Variables|Default|Getstring1) (Math|Transform|MakeTransform (* (+ CenterPosition _returnvalue_3) 0.5) (Math|Rotator|FindLookatRotation CenterPosition _returnvalue_3) (Math|Vector|MakeVector (* (Math|Vector|VectorLength (- CenterPosition _returnvalue_3)) 0.01) _returnvalue _returnvalue)) false false))
    (:then_1
      ;[1 1 1] update the arrow
      (if (> (Math|Vector|VectorLength (- CenterPosition (* (+ (Transformation|GetWorldLocation (Variables|Default|Getend1)) (Transformation|GetWorldLocation (Variables|Default|Getend2))) 0.5))) 15.0)
        (Utilities|FlowControl|DoOnce false
          (:Completed
            (CallFunction|SpawnArrow CenterPosition)))))
    (:then_2
      (CallFunction|UpdateArrow CenterPosition))))

(event Custom|ResetArrowSpawn
  ;[1 1 1] update the arrow
  (Utilities|FlowControl|DoOnce false) ; enters at Reset
)

(event Custom|UpdateArrow
  (params (HandPosition :type Vector))
  (bind _spawnedarrows (Variables|Default|GetSpawnedArrows))
  ;[1 1 1] arrow
  (if (Variables|NotUsed|GetNextShotIsMultiShot)
    (if (> (Utilities|Array|Length (Variables|Default|GetSpawnedArrows)) 0)
      (for (_array_element _array_index) (Variables|NotUsed|GetMutliShotXOffset)
        (Transformation|SetActorTransform (Utilities|Array|Get(acopy) (Variables|Default|GetSpawnedArrows) _array_index) (Math|Transform|MakeTransform HandPosition (Math|Rotator|FindLookatRotation HandPosition (Math|Transform|TransformLocation (Transformation|GetActorTransform) (Math|Vector|MakeVector _array_element 0.0 0.0))) "2.000000,2.000000,2.000000"))))
    (elif (> (Utilities|Array|Length _spawnedarrows) 0)
      (Transformation|SetActorTransform (Utilities|Array|Get(acopy) _spawnedarrows) (Math|Transform|MakeTransform HandPosition (Math|Rotator|FindLookatRotation HandPosition (Transformation|GetWorldLocation (Variables|Default|GetArrowAttatchPoint))) "2.000000,2.000000,2.000000")))))

(event Custom|ReleaseString
  (params (ReleasePosition :type Vector))
  (Utilities|FlowControl|Sequence
    (:then_0
      ;[1 1 1] shoot arrow if have
      (Variables|NotUsed|SetNextShotIsMultiShot false)
      (for _array_element (Variables|Default|GetSpawnedArrows)
        (Transformation|DetachFromActor _array_element "KeepWorld" "KeepWorld" "KeepWorld")
        (Variables|/Script/Engine.MovementComponent|SetVelocity (Variables|/Game/ClashRoyaleTest/Blueprints/SpawnObject/Bullet/WeaponBullet/BP_Bow_Bullet.BP_Bow_Bullet_C|GetProjectileMovement _array_element) (* (Math|Vector|GetForwardVector (Variables|/Game/ClashRoyaleTest/Blueprints/SpawnObject/Bullet/WeaponBullet/BP_Bow_Bullet.BP_Bow_Bullet_C|GetStaticMesh _array_element)) (Math|Vector|VectorLength (* (- (* (+ (Transformation|GetWorldLocation (Variables|Default|Getend1)) (Transformation|GetWorldLocation (Variables|Default|Getend2))) 0.5) ReleasePosition) 5e+01))))
        (Components|Activation|SetActive (Variables|/Game/ClashRoyaleTest/Blueprints/SpawnObject/Bullet/WeaponBullet/BP_Bow_Bullet.BP_Bow_Bullet_C|GetProjectileMovement _array_element) true false)
        (Actor|SetLifeSpan _array_element 5.0)
        (Collision|IgnoreActorwhenMoving (Variables|/Game/ClashRoyaleTest/Blueprints/SpawnObject/Bullet/WeaponBullet/BP_Bow_Bullet.BP_Bow_Bullet_C|GetStaticMesh _array_element) (Components|GetOwner self) true)
        (bind _outactors (Actor|GetAllActorsOfClass "/Game/ClashRoyaleTest/Blueprints/SpawnObject/Bullet/WeaponBullet/BP_Bow_Bullet.BP_Bow_Bullet_C"))
        (for _array_element_2 _outactors
          (Collision|IgnoreActorwhenMoving (Variables|/Game/ClashRoyaleTest/Blueprints/SpawnObject/Bullet/WeaponBullet/BP_Bow_Bullet.BP_Bow_Bullet_C|GetStaticMesh _array_element) _array_element_2 true)))
      (Utilities|Array|Clear (Variables|Default|GetSpawnedArrows)))
    (:then_1
      ;[1 1 1] update string
      (bind _lerp (Timeline|ReleaseStringTimeLine PlayFromStart)
        (:Update
          (CallFunction|UpdateString (Math|Vector|Lerp(Vector) ReleasePosition (* (+ (Transformation|GetWorldLocation (Variables|Default|Getend1)) (Transformation|GetWorldLocation (Variables|Default|Getend2))) 0.5) _lerp)))
        (:Finished
          (CallFunction|ResetArrowSpawn))))))

(event Custom|SpawnArrow
  (params (HandPosition :type Vector))
  ;[1 1 1] arrow
  (if (Variables|NotUsed|GetNextShotIsMultiShot)
    (for _array_element (Variables|NotUsed|GetMutliShotXOffset)
      (bind _returnvalue (Game|SpawnActorfromClass "/Game/ClashRoyaleTest/Blueprints/SpawnObject/Bullet/WeaponBullet/BP_Bow_Bullet.BP_Bow_Bullet_C" (Math|Transform|MakeTransform HandPosition (Math|Rotator|FindLookatRotation HandPosition (Math|Transform|TransformLocation (Transformation|GetActorTransform) (Math|Vector|MakeVector _array_element 0.0 0.0))) "2.000000,2.000000,2.000000") "Undefined" (.AsPawn (Utilities|Casting|CastToPawn (Components|GetOwner self))) 0))
      (Actor|SetLifeSpan 0.0)
      (Collision|IgnoreActorwhenMoving (Variables|/Game/ClashRoyaleTest/Blueprints/SpawnObject/Bullet/WeaponBullet/BP_Bow_Bullet.BP_Bow_Bullet_C|GetStaticMesh _returnvalue) self true)
      (Utilities|Array|Add (Variables|Default|GetSpawnedArrows) _returnvalue))
    (else
      (bind _returnvalue_2 (Game|SpawnActorfromClass "/Game/ClashRoyaleTest/Blueprints/SpawnObject/Bullet/WeaponBullet/BP_Bow_Bullet.BP_Bow_Bullet_C" (Math|Transform|MakeTransform HandPosition (Math|Rotator|FindLookatRotation HandPosition (Transformation|GetWorldLocation (Variables|Default|GetArrowAttatchPoint))) "2.000000,2.000000,2.000000") "Undefined" (.AsPawn (Utilities|Casting|CastToPawn (Components|GetOwner self))) 0))
      (Actor|SetLifeSpan 0.0)
      (Collision|IgnoreActorwhenMoving (Variables|/Game/ClashRoyaleTest/Blueprints/SpawnObject/Bullet/WeaponBullet/BP_Bow_Bullet.BP_Bow_Bullet_C|GetStaticMesh _returnvalue_2) self true)
      (Utilities|Array|Add (Variables|Default|GetSpawnedArrows) _returnvalue_2))))

(event EventOnPickup
  (params (Interactor :type World%20Interactor%20Object%20Reference))
  (bind _bowmesh (Variables|Default|GetBowMesh))
  ;[1 1 1] bow physics
  (Physics|SetEnableGravity _bowmesh false)
  (Variables|Default|SetPreviousLinearDamping (Class|PrimitiveComponent|GetLinearDamping _bowmesh))
  (Variables|Default|SetPreviousAngularDamping (Class|PrimitiveComponent|GetAngularDamping _bowmesh))
  (Class|PrimitiveComponent|SetLinearDamping _bowmesh 9999999999.0)
  (Class|PrimitiveComponent|SetAngularDamping _bowmesh 99999999.0)
  (Variables|Default|SetIsPickuped true))

(event EventOnDrag
  (params (Interactor :type World%20Interactor%20Object%20Reference))
  (if (Variables|Default|GetIsPulling)
    (CallFunction|UpdateString (Transformation|GetWorldLocation Interactor))))

(event EventOnDragEnd
  (params (Interactor :type World%20Interactor%20Object%20Reference))
  (if (Variables|Default|GetIsPulling)
    (CallFunction|ReleaseString (Transformation|GetWorldLocation Interactor))
    (Variables|Default|SetIsPulling false)))

(event EventOnDrop
  (params (Velocity :type Vector) (AngularVelocity :type Vector) (Interactor :type World%20Interactor%20Object%20Reference))
  (bind _bowmesh (Variables|Default|GetBowMesh))
  ;[1 1 1] bow physics
  (Class|PrimitiveComponent|SetLinearDamping _bowmesh (Variables|Default|GetPreviousLinearDamping))
  (Class|PrimitiveComponent|SetAngularDamping _bowmesh (Variables|Default|GetPreviousAngularDamping))
  (Physics|SetEnableGravity _bowmesh true)
  (Physics|AddImpulse _bowmesh Velocity "None" true)
  (Class|PrimitiveComponent|AddAngularImpulse _bowmesh AngularVelocity "None" true)
  (Variables|Default|SetIsPickuped false))

(event EventOnDragStart
  (params (Interactor :type World%20Interactor%20Object%20Reference))
  (if (Variables|Default|GetIsPickuped)
    (bind _outcomponents (Class|KismetSystemLibrary|SphereOverlapComponentsNEW (Transformation|GetWorldLocation Interactor) 1e+01 (Utilities|Array|MakeArray "ObjectTypeQuery2") "/Script/Engine.SphereComponent"))
    (if (> (Utilities|Array|Length _outcomponents) 0)
      (if (Components|ComponentHasTag (Utilities|Array|Get(acopy) _outcomponents) "Emitter")
        (Variables|Default|SetIsPulling true)))))

(fn ConstructionScript
  (CallFunction|UpdateString (* (+ (Transformation|GetWorldLocation (Variables|Default|Getend1)) (Transformation|GetWorldLocation (Variables|Default|Getend2))) 0.5)))

(fn CanDrop
  (return false))

(fn CanPickup
  (return false))

(fn GetAttachLocation
  (return "3.923019,0.000114,-19.554785"))

(fn GetAttachRotation
  (return "0,180.000000,-180.000000"))

(fn ShouldSnaptoInteractor
  (return true))