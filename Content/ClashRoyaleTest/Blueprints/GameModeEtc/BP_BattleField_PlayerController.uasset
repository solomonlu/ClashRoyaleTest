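; Player controller for the battlefield in a Clash Royale-style test project, managing the player's energy resource.
; Each tick, DealEnergy regenerates CurEnergy at EnergyRecoverSpeed while it is below MaxEnergy.
; A ConsumeEnergy event subtracts a given amount, and both paths clamp the value between zero and the maximum.
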(event Custom|ConsumeEnergy
  (params (Energy :type Float%20%28single-precision%29))
  (Variables|Energy|SetCurEnergy (Math|Float|Clamp(Float) (- (Variables|Energy|GetCurEnergy) Energy) 0.0 (Math|Conversions|ToFloat(Integer) (Variables|Energy|GetMaxEnergy)))))

(event EventTick
  (params (DeltaSeconds :type Float%20%28single-precision%29))
  (CallFunction|DealEnergy DeltaSeconds))

(fn ConstructionScript)

(fn DealEnergy
  (params (DeltaTime :type Float%20%28single-precision%29))
  ;[1 1 1] recover energy all the time
  (if (< (Variables|Energy|GetCurEnergy) (Math|Conversions|ToFloat(Integer) (Variables|Energy|GetMaxEnergy)))
    (Variables|Energy|SetCurEnergy (Math|Float|Clamp(Float) (+ (Variables|Energy|GetCurEnergy) (* DeltaTime (Variables|Energy|GetEnergyRecoverSpeed))) 0.0 (Math|Conversions|ToFloat(Integer) (Variables|Energy|GetMaxEnergy)))))
  (return))