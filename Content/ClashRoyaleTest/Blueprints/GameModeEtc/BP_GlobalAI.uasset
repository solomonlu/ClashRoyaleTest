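; BP_GlobalAI is an automatic skill-ball spawner that, while active, launches random balls for its Camp on a looping timer, optionally also shortly after BeginPlay.
; Each spawn picks a name from RandomSkillBallNameList, reads its DT_SkillBall row and spawns that class at SpawnPoint relative to the actor.
; It passes energy cost and split count through BPI_SkillBallInterface, then toggles projectile movement.
; SpawnBoxExtent randomizes launch velocity, not location, and also sizes the optional debug box.
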(event Custom|SpawnRandomActor
  (bind _randomskillballnamelist (Variables|Default|GetRandomSkillBallNameList))
  (Utilities|FlowControl|Sequence
    (:then_0
      ;[1 1 1] debug
      (if (Variables|Default|GetShowDebugBox)
        (Rendering|Debug|DrawDebugBox (Math|Transform|TransformLocation (Transformation|GetActorTransform) (Variables|Default|GetSpawnPoint)) (Variables|Default|GetSpawnBoxExtent) "(R=0.000000,G=1.000000,B=0.000000,A=1.000000)" "0, 0, 0" (Variables|Default|GetSpawnInterval) 1.0)))
    (:then_1
      (bind _returnvalue (Utilities|GetDataTableRow "/Game/ClashRoyaleTest/Blueprints/GameDesign/DT_SkillBall.DT_SkillBall" (Utilities|String|StringToName (Utilities|Array|Get(acopy) _randomskillballnamelist (Math|Random|RandomIntegerinRange 0 (Utilities|Array|LastIndex _randomskillballnamelist)))))
        (:then
          (bind _returnvalue_2 (Game|SpawnActorfromClass (.Class (Utilities|Struct|BreakS_SkillBallDataTable _returnvalue)) (Math|Transform|MakeTransform (Math|Transform|TransformLocation (Transformation|GetActorTransform) (Variables|Default|GetSpawnPoint)) "0, 0, 0" "1,1,1") "Undefined" 0 0))
          (Utilities|FlowControl|Sequence
            (:then_0
              (if (Utilities|DoesObjectImplementInterface _returnvalue_2 "/Game/ClashRoyaleTest/Blueprints/SkillBall/BPI_SkillBallInterface.BPI_SkillBallInterface_C")
                (Class|BPISkillBallInterface|SetSkillBallEnergyCost(Message) _returnvalue_2 (.EnergyCost (Utilities|Struct|BreakS_SkillBallDataTable _returnvalue)))
                (Class|BPISkillBallInterface|SetSkillBallSplitCount(Message) _returnvalue_2 (.SpawnSoldiersCount (Utilities|Struct|BreakS_SkillBallDataTable _returnvalue)))))
            (:then_1
              (bind _asbp_skill_ball_base (Utilities|Casting|CastToBP_SkillBall_Base _returnvalue_2))
              (Variables|/Game/ClashRoyaleTest/Blueprints/SkillBall/BP_SkillBall_Base.BP_SkillBall_Base_C|SetCamp _asbp_skill_ball_base (Variables|Default|GetCamp))
              (if (> (Utilities|Array|Length (Actor|GetComponentsByClass _returnvalue_2 "/Script/Engine.ProjectileMovementComponent")) 0)
                (Components|Activation|ToggleActive (Utilities|Array|Get(acopy) (Actor|GetComponentsByClass _returnvalue_2 "/Script/Engine.ProjectileMovementComponent")))
                (Variables|/Script/Engine.MovementComponent|SetVelocity (Utilities|Array|Get(acopy) (Actor|GetComponentsByClass _returnvalue_2 "/Script/Engine.ProjectileMovementComponent")) (Math|Random|RandomPointinBoundingBox (Math|Vector|MakeVector 0.0 0.0 0.0) (Variables|Default|GetSpawnBoxExtent)))))))))))

(event EventBeginPlay
  (if (Variables|Default|GetIsActive)
    (Utilities|Time|SetTimerbyEvent (delegate Custom|SpawnRandomActor) (Variables|Default|GetSpawnInterval) true)
    (if (Variables|Default|GetSpawnAtOnce)
      (Utilities|FlowControl|Delay 0.5)
      (CallFunction|SpawnRandomActor))))

(fn ConstructionScript)